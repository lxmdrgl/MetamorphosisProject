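; Screwdriver pickup that the player interacts with to add the tool to the first-person character.
; BeginPlay sets the interaction prompt, caches the character and adds a WB_ViewText widget to the viewport.
; Interact notifies the character, disables further interaction, removes the screwdriver component and shows usage hints briefly before removing the widget and destroying the actor.
; The construction script applies a configurable scale to the screwdriver in the editor.
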(event `self.ReceiveBeginPlay`
  ;[0.681 1 0] Set Up Scene
  (set `self.InteractName` "pick up screwdriver")
  (bind _asbp_first_person_character (cast `/Game/FirstPerson/Blueprints/BP_FirstPersonCharacter` (`GameplayStatics.GetPlayerCharacter` 0)))
  (set `self.BP_CharRef` _asbp_first_person_character)
  (bind _returnvalue (`|CreateWidget` "/Game/Blueprints/Interact/WB_ViewText.WB_ViewText_C"))
  (bind _output_get (set `self.WidgetRef` _returnvalue))
  (`UserWidget.AddToViewport` _output_get 0))

(event `/Game/Blueprints/Interact/Interface_Interact.Interact`
  (params (SMRef :type "StaticMeshComponent Object Reference"))
  (bind _widgetref (`self.WidgetRef`))
  (bind _widgetref_2 (`self.WidgetRef`))
  ;[0.2336 0 1] Interact
  (`/Game/FirstPerson/Blueprints/BP_FirstPersonCharacter.ScrewdriverPickedUp` (`self.BP_CharRef`))
  (set `self.CanInteract` false)
  (`ActorComponent.K2_DestroyComponent` (`self.screwdriver`))
  (set `/Game/Blueprints/Interact/WB_ViewText.Name_2` "Use screwdriver to interact with certain items" _widgetref)
  (set `/Game/Blueprints/Interact/WB_ViewText.Name_4` "Press 1 to switch hand to screwdriver" _widgetref)
  (`KismetSystemLibrary.Delay` 10.0)
  (set `/Game/Blueprints/Interact/WB_ViewText.Name_2` "" _widgetref_2)
  (set `/Game/Blueprints/Interact/WB_ViewText.Name_4` "" _widgetref_2)
  (`Widget.RemoveFromParent` _widgetref_2)
  (`self.K2_DestroyActor`))

(event `ChangeScrewdriverScale`
  ;[1 0.0154 0] Edit Scale From Editor
  (`SceneComponent.SetRelativeScale3D` (`self.screwdriver`) (`KismetMathLibrary.Conv_DoubleToVector` (`self.ScrewdriverScale`))))

(fn `UserConstructionScript`
  (`parent.UserConstructionScript`)
  (`self.ChangeScrewdriverScale`))