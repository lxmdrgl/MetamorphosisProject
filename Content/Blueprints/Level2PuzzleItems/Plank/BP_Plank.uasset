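; BP_Plank is a Level 2 puzzle board that the player cuts by holding interact while the saw is enabled.
; Each Tick, a short line trace from the first-person camera toggles input and CanInteract, based on looking at this plank with the saw.
; IA_Interact's elapsed time fills a WB_ProgressBar widget created on BeginPlay, resetting on cancel.
; When the action triggers, interaction locks and the plank destroys itself.
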(event `self.ReceiveBeginPlay`
  (bind _asbp_first_person_character (cast `/Game/FirstPerson/Blueprints/BP_FirstPersonCharacter` (`GameplayStatics.GetPlayerCharacter` 0)))
  (set `self.FPCharRef` _asbp_first_person_character)
  (set `self.InteractName` "cut board")
  (bind _returnvalue (`|CreateWidget` "/Game/Blueprints/Interact/WB_ProgressBar.WB_ProgressBar_C"))
  (bind _output_get (set `self.WidgetRef` _returnvalue))
  (`UserWidget.AddToViewport` _output_get 0))

(event `self.ReceiveTick`
  (params (DeltaSeconds :type "Float (single-precision)"))
  (bind _returnvalue (`GameplayStatics.GetPlayerController` 0))
  (bind _firstpersoncamera (`/Game/FirstPerson/Blueprints/BP_FirstPersonCharacter.FirstPersonCamera` (`self.FPCharRef`)))
  (bind _returnvalue_2 (`SceneComponent.K2_GetComponentLocation` _firstpersoncamera))
  (bind (_outhit _returnvalue_3) (`KismetSystemLibrary.LineTraceSingle` :`Start` _returnvalue_2 :`End` (+ _returnvalue_2 (* (`SceneComponent.GetForwardVector` _firstpersoncamera) 200.0)) :`TraceChannel` "TraceTypeQuery1" :`bIgnoreSelf` false :`DrawTime` 1.0))
  (bind _output_get (set `self.IsViewBoard` _returnvalue_3))
  (if _output_get
    (if (== (`.HitActor` (`GameplayStatics.BreakHitResult` _outhit)) self)
      (if (`self.InteractOver`)
        (`self.DisableInput` _returnvalue null :!label _label)
        (set `self.CanInteract` false)
        (elif (`/Game/FirstPerson/Blueprints/BP_FirstPersonCharacter.IsSawEnabled` (`self.FPCharRef`))
          (`self.EnableInput` _returnvalue)
          (set `self.CanInteract` true)
          (else
            (goto _label))))
      (else
        (`|ExecutionSequence`
          (:`then_0`
            (goto _label)))))
    (else
      (goto _label))))

(event `EnhancedInput|/Game/FirstPerson/Input/Actions/IA_Interact`
  (params (ActionValue :type Boolean) (ElapsedSeconds :type "Float (double-precision)") (TriggeredSeconds :type "Float (double-precision)") (InputAction :type "InputAction Object Reference" :default "/Game/FirstPerson/Input/Actions/IA_Interact.IA_Interact"))
  (bind _interactover (`self.InteractOver`))
  (:`Triggered`
    (set `self.InteractOver` true)
    (set `/Game/Blueprints/Interact/WB_ProgressBar.Percent` 0.0 (`self.WidgetRef`))
    (`/Engine/EditorBlueprintResources/StandardMacros.DoOnce` false
      (:`Completed`
        (`self.K2_DestroyActor`))))
  (:`Ongoing`
    (if (`self.CanInteract`)
      (if (not _interactover)
        (set `/Game/Blueprints/Interact/WB_ProgressBar.Percent` (/ ElapsedSeconds 5.0) (`self.WidgetRef`)))))
  (:`Canceled`
    (if (not _interactover)
      (set `/Game/Blueprints/Interact/WB_ProgressBar.Percent` 0.0 (`self.WidgetRef`)))))

(fn `UserConstructionScript`)