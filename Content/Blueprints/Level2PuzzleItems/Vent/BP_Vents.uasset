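; BP_Vents is a vent puzzle item whose door moves to an end position once the screw condition is met.
; Every tick it counts all BP_Screw actors in the level, and when exactly three exist a DoOnce fires FinishedScrews.
; That event plays the T_DoorFall timeline, lerping the VentDoor's relative location from start to end without sweeping.
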(event `self.ReceiveTick`
  (params (DeltaSeconds :type "Float (single-precision)"))
  (bind _outactors (`GameplayStatics.GetAllActorsOfClass` "/Game/Blueprints/Level2PuzzleItems/Vent/BP_Screw.BP_Screw_C"))
  (bind _output_get (set `self.ScrewCount` (`KismetArrayLibrary.Array_Length` _outactors)))
  (if (== _output_get 3)
    (`/Engine/EditorBlueprintResources/StandardMacros.DoOnce` false
      (:`Completed`
        (`self.FinishedScrews`)))))

(event `FinishedScrews`
  (bind (_direction _alpha) (`Timeline|T_DoorFall` :!via `PlayFromStart`)
    (:`Update`
      (`SceneComponent.K2_SetRelativeLocation` (`self.VentDoor`) (`KismetMathLibrary.VLerp` (`self.StartDoorLocation`) (`self.EndDoorLocation`) _alpha) false false))))

(fn `UserConstructionScript`)