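; BP_Plush is an interactable plush among the Level 2 puzzle items that animates its Top part when used.
; BeginPlay sets its interaction prompt name and speeds up the transform timeline.
; Interacting sets InteractOver and plays the timeline from the start, lerping Top's relative transform from StartTransform to EndTransform.
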(event `self.ReceiveBeginPlay`
  (set `self.InteractName` "interact with plush")
  (`TimelineComponent.SetPlayRate` (`self.T_Transform`) 2.0))

(event `/Game/Blueprints/Interact/Interface_Interact.Interact`
  (params (SMRef :type "StaticMeshComponent Object Reference"))
  (set `self.InteractOver` true)
  (bind (_direction _alpha) (`Timeline|T_Transform` :!via `PlayFromStart`)
    (:`Update`
      (`SceneComponent.K2_SetRelativeTransform` (`self.Top`) (`KismetMathLibrary.TLerp` (`self.StartTransform`) (`self.EndTransform`) _alpha) false false))))

(fn `UserConstructionScript`)