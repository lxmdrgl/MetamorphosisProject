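; BP_Pipe_3 is an interactable pipe for a Level 2 puzzle that toggles between two orientations.
; Each interaction flips IsStartingPosition and plays a timeline forward or in reverse, lerping the root's roll a quarter turn.
; Interaction is locked during the rotation; on finish it unlocks and tells the BP_Vents actor to update pipe orientation.
; The construction script sets the starting rotation.
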(event `self.ReceiveBeginPlay`
  (set `self.InteractName` "change pipe orientation")
  (`TimelineComponent.SetPlayRate` (`self.T_RotatePipe`) 1.0))

(event `/Game/Blueprints/Interact/Interface_Interact.Interact`
  (params (SMRef :type "StaticMeshComponent Object Reference"))
  (set `self.CanInteract` false)
  (if (`self.IsStartingPosition`)
    (set `self.IsStartingPosition` false)
    (bind (_direction _alpha) (`Timeline|T_RotatePipe` :!via `PlayFromStart` :!label _label)
      (:`Update`
        (`SceneComponent.K2_SetRelativeRotation` (`self.DefaultSceneRoot`) (`KismetMathLibrary.MakeRotator` (`KismetMathLibrary.Lerp` 180.0 90.0 _alpha) 0.0 180.0) false false))
      (:`Finished`
        (set `self.CanInteract` true)
        (bind _returnvalue (`GameplayStatics.GetActorOfClass` "/Game/Blueprints/Level2PuzzleItems/Vent/BP_Vents.BP_Vents_C"))
        (`/Game/Blueprints/Level2PuzzleItems/Vent/BP_Vents.UpdatePipeOrientation` _returnvalue)))
    (else
      (set `self.IsStartingPosition` true)
      (goto _label :!via `ReverseFromEnd`))))

(fn `UserConstructionScript`
  (`SceneComponent.K2_SetRelativeRotation` (`self.DefaultSceneRoot`) (`KismetMathLibrary.MakeRotator` 180.0 0.0 180.0) false false))