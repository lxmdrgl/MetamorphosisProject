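; BP_FlashlightPickup is an interactable world item that gives the player the flashlight.
; BeginPlay sets the interaction prompt, caches the first-person character and adds a WB_ViewText widget to the viewport.
; Interact tells the character the flashlight was picked up, disables further interaction and removes the mesh.
; It then shows control hints through the widget for a short time before removing the widget and destroying itself.
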(event `self.ReceiveBeginPlay`
  (set `self.InteractName` "pickup flashlight")
  (bind _asbp_first_person_character (cast `/Game/FirstPerson/Blueprints/BP_FirstPersonCharacter` (`GameplayStatics.GetPlayerCharacter` 0)))
  (set `self.BPCharRef` _asbp_first_person_character)
  (bind _returnvalue (`|CreateWidget` "/Game/Blueprints/Interact/WB_ViewText.WB_ViewText_C"))
  (bind _output_get (set `self.WidgetRef` _returnvalue))
  (`UserWidget.AddToViewport` _output_get 0))

(event `/Game/Blueprints/Interact/Interface_Interact.Interact`
  (params (SMRef :type "StaticMeshComponent Object Reference"))
  (bind _widgetref (`self.WidgetRef`))
  (bind _widgetref_2 (`self.WidgetRef`))
  (`/Game/FirstPerson/Blueprints/BP_FirstPersonCharacter.FlashlightPickedUp` (`self.BPCharRef`))
  (set `self.CanInteract` false)
  (`ActorComponent.K2_DestroyComponent` (`self.StaticMesh`))
  (set `/Game/Blueprints/Interact/WB_ViewText.Name_2` "Press Left Click to use flashlight" _widgetref)
  (set `/Game/Blueprints/Interact/WB_ViewText.Name_4` "Press 1 to switch hand to flashlight" _widgetref)
  (`KismetSystemLibrary.Delay` 10.0)
  (set `/Game/Blueprints/Interact/WB_ViewText.Name_2` "" _widgetref_2)
  (set `/Game/Blueprints/Interact/WB_ViewText.Name_4` "" _widgetref_2)
  (`Widget.RemoveFromParent` (`self.WidgetRef`))
  (`self.K2_DestroyActor`))

(fn `UserConstructionScript`)