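; BP_Saw is a world pickup that gives the first-person character a saw.
; On BeginPlay it sets its interact prompt, caches the player character and adds a WB_ViewText widget to the viewport.
; Interact notifies the character of the pickup, disables further interaction and removes the saw component.
; It then shows usage and hand-switch hints for a few seconds before removing the widget and destroying itself.
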(event `self.ReceiveBeginPlay`
  (set `self.InteractName` "pickup saw")
  (bind _asbp_first_person_character (cast `/Game/FirstPerson/Blueprints/BP_FirstPersonCharacter` (`GameplayStatics.GetPlayerCharacter` 0)))
  (set `self.FPCharRef` _asbp_first_person_character)
  (bind _returnvalue (`|CreateWidget` "/Game/Blueprints/Interact/WB_ViewText.WB_ViewText_C"))
  (bind _output_get (set `self.WidgetRef` _returnvalue))
  (`UserWidget.AddToViewport` _output_get 0))

(event `/Game/Blueprints/Interact/Interface_Interact.Interact`
  (params (SMRef :type "StaticMeshComponent Object Reference"))
  (bind _widgetref (`self.WidgetRef`))
  (bind _widgetref_2 (`self.WidgetRef`))
  (`/Game/FirstPerson/Blueprints/BP_FirstPersonCharacter.SawPickedUp` (`self.FPCharRef`))
  (set `self.CanInteract` false)
  (`ActorComponent.K2_DestroyComponent` (`self.Saw`))
  (set `/Game/Blueprints/Interact/WB_ViewText.Name_2` "Use saw on certain items" _widgetref)
  (set `/Game/Blueprints/Interact/WB_ViewText.Name_4` "Press 3 to switch hand to saw" _widgetref)
  (`KismetSystemLibrary.Delay` 5.0)
  (set `/Game/Blueprints/Interact/WB_ViewText.Name_2` "" _widgetref_2)
  (set `/Game/Blueprints/Interact/WB_ViewText.Name_4` "" _widgetref_2)
  (`Widget.RemoveFromParent` (`self.WidgetRef`))
  (`self.K2_DestroyActor`))

(fn `UserConstructionScript`)