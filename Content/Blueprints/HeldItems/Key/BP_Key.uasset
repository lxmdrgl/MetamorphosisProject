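; BP_Key is an interactable key item, apparently unfinished, with prompt text that refers to a flashlight.
; On BeginPlay it sets its interact name, caches the first-person character and adds a WB_ViewText widget to the viewport.
; Its Interact event is empty.
; A disconnected pickup chain would remove the key component, show timed flashlight hints, then destroy the actor, but it never runs.
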(event `self.ReceiveBeginPlay`
  (set `self.InteractName` "pickup flashlight")
  (bind _asbp_first_person_character (cast `/Game/FirstPerson/Blueprints/BP_FirstPersonCharacter` (`GameplayStatics.GetPlayerCharacter` 0)))
  (set `self.FPCharRef` _asbp_first_person_character)
  (bind _returnvalue (`|CreateWidget` "/Game/Blueprints/Interact/WB_ViewText.WB_ViewText_C"))
  (bind _output_get (set `self.WidgetRef` _returnvalue))
  (`UserWidget.AddToViewport` _output_get 0))

(event `/Game/Blueprints/Interact/Interface_Interact.Interact`
  (params (SMRef :type "StaticMeshComponent Object Reference")))

(fn `UserConstructionScript`)