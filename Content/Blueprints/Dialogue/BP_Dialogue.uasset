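; BP_Dialogue plays scripted dialogue scenes from DT_Dialogue and shows their text through a WB_Dialogue widget.
; PlayScene finds the row matching a scene index, then steps through its lines, playing each sound and delaying for its duration unless SkipDialogue is set.
; When lines run out, it fires that scene's end event, calling the Gregor desk or cutscene collision actor for Level1 scenes.
; Scene one starts from an event bound on the desk actor at BeginPlay.
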(event `PlayScene`
  (params (Index :type Integer))
  (set `self.DTIndex` Index)
  (bind _outrownames (`DataTableFunctionLibrary.GetDataTableRowNames` "/Game/Blueprints/Dialogue/DT_Dialogue.DT_Dialogue"))
  (for (_array_element _array_index) _outrownames
    (if (== _array_index (`self.DTIndex`))
      (bind _returnvalue (`|GetDataTableRow` "/Game/Blueprints/Dialogue/DT_Dialogue.DT_Dialogue" _array_element)
        (:`then`
          (set `self.CurrIndex` 0)
          (set `self.DialogueArrayRef` (`.Dialogue_3_E1D8773840C52B4142EABCAF99F32B1A` (break `/Game/Blueprints/Dialogue/S_Scene` _returnvalue)))
          (if (not (`self.SkipDialogue`)) :!label _label
            (bind (_sound _text) (break `/Game/Blueprints/Dialogue/S_Dialogue` (`|GetArrayItem` (`.Dialogue_3_E1D8773840C52B4142EABCAF99F32B1A` (break `/Game/Blueprints/Dialogue/S_Scene` _returnvalue)) (`self.CurrIndex`))))
            (`GameplayStatics.PlaySound2D` _sound 1.0 1.0 0.0 null null))
          (set `/Game/Blueprints/Dialogue/WB_Dialogue.Text` _text (`self.WidgetRef`))
          (if (not (`self.SkipDialogue`))
            (`KismetSystemLibrary.Delay` (`SoundBase.Duration` _sound)))
          (`/Engine/EditorBlueprintResources/StandardMacros.IncrementInt` (`self.CurrIndex`)
            (:`  `
              (if (`KismetArrayLibrary.Array_IsValidIndex` (`self.DialogueArrayRef`) (`self.CurrIndex`))
                (goto _label)
                (else
                  (set `/Game/Blueprints/Dialogue/WB_Dialogue.Text` "" (`self.WidgetRef`))
                  (`|ExecutionSequence`
                    (:`then_0`
                      (if (== (`self.DTIndex`) 0)
                        (`self.EndScene1`)))
                    (:`then_1`
                      (if (== (`self.DTIndex`) 1)
                        (if (`self.Level_1`)
                          (bind _returnvalue_2 (`GameplayStatics.GetActorOfClass` "/Game/Blueprints/Desk/Desk_Main/BP_S2_GregorDesk.BP_S2_GregorDesk_C"))
                          (`/Game/Blueprints/Desk/Desk_Main/BP_S2_GregorDesk.EndScene2` _returnvalue_2))))
                    (:`then_2`
                      (if (== (`self.DTIndex`) 2)
                        (if (`self.Level_1`)
                          (bind _returnvalue_3 (`GameplayStatics.GetActorOfClass` "/Game/Blueprints/CutsceneCollision/BP_CutsceneCollision_1.BP_CutsceneCollision_1_C"))
                          (`/Game/Blueprints/CutsceneCollision/BP_CutsceneCollision_1.EndScene3` _returnvalue_3))))
                    (:`then_3`
                      (if (== (`self.DTIndex`) 3)
                        (if (`self.Level_1`)
                          (bind _returnvalue_4 (`GameplayStatics.GetActorOfClass` "/Game/Blueprints/CutsceneCollision/BP_CutsceneCollision_1.BP_CutsceneCollision_1_C"))
                          (`/Game/Blueprints/CutsceneCollision/BP_CutsceneCollision_1.EndScene4` _returnvalue_4))))))))))))))

(event `self.ReceiveBeginPlay`
  (`|ExecutionSequence`
    (:`then_0`
      (bind _returnvalue (`|CreateWidget` "/Game/Blueprints/Dialogue/WB_Dialogue.WB_Dialogue_C"))
      (bind _output_get (set `self.WidgetRef` _returnvalue))
      (`UserWidget.AddToViewport` _output_get 0))
    (:`then_1`
      (bind _returnvalue_2 (`GameplayStatics.GetActorOfClass` "/Game/Blueprints/Desk/Desk_Main/BP_S2_GregorDesk.BP_S2_GregorDesk_C"))
      (add `/Game/Blueprints/Desk/Desk_Main/BP_S2_GregorDesk.PlayScene1` _returnvalue_2 (delegate `PlaySceneOne`)))))

(event `PlaySceneOne`
  (`self.PlayScene` 0))

(fn `UserConstructionScript`)