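; BP_DoorHold is a door the player holds shut with Interact while inside its sphere, or lights with a flashlight when not holding it.
; Overlap shows hint text and animates the player's flashlight into view; leaving hides it and releases the door.
; A timeline lerps door yaw toward closed and reverses on release.
; BP_Father is notified when the door fully closes and when it is released afterward.
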(event `self.ReceiveBeginPlay`
  (bind _pfcharref (`self.PFCharRef`))
  (bind _asbp_first_person_character (cast `/Game/FirstPerson/Blueprints/BP_FirstPersonCharacter` (`GameplayStatics.GetPlayerCharacter` 0)))
  (set `self.PFCharRef` _asbp_first_person_character)
  (bind _returnvalue (`|CreateWidget` "/Game/Blueprints/Interact/WB_ViewText.WB_ViewText_C"))
  (bind _output_get (set `self.WidgetRef` _returnvalue))
  (`UserWidget.AddToViewport` _output_get 0)
  (`self.EnableInput` (`GameplayStatics.GetPlayerController` 0))
  (set `self.FlashlightRef` (`/Game/FirstPerson/Blueprints/BP_FirstPersonCharacter.FlashlightBetter` _pfcharref))
  (set `self.LightRef` (`/Game/FirstPerson/Blueprints/BP_FirstPersonCharacter.SpotLight` _pfcharref)))

(event `self.Sphere.OnComponentBeginOverlap`
  (params (OverlappedComponent :type "PrimitiveComponent Object Reference") (OtherActor :type "Actor Object Reference") (OtherComp :type "PrimitiveComponent Object Reference") (OtherBodyIndex :type Integer) (bFromSweep :type Boolean) (SweepResult :type "HitResult Structure (by ref)"))
  (bind _widgetref (`self.WidgetRef`))
  (bind _relativescale3d (`SceneComponent.RelativeScale3D` (`self.FlashlightRef`)))
  (set `self.InCollision` true)
  (set `/Game/Blueprints/Interact/WB_ViewText.Name` "Hold E to close door" _widgetref)
  (set `/Game/Blueprints/Interact/WB_ViewText.Name_2` "Press Left Click to use flashlight" _widgetref)
  (`SceneComponent.SetVisibility` (`self.FlashlightRef`) true false)
  (`SceneComponent.K2_SetRelativeTransform` (`self.FlashlightRef`) (`KismetMathLibrary.MakeTransform` (`self.StartFlashlightLocation`) (`self.StartFlashlightRotation`) _relativescale3d) false false)
  (`TimelineComponent.SetPlayRate` (`self.T_Flashlight`) 2.0)
  (bind (_direction _alpha) (`Timeline|T_Flashlight` :!via `PlayFromStart`)
    (:`Update`
      (`SceneComponent.K2_SetRelativeTransform` (`self.FlashlightRef`) (`KismetMathLibrary.TLerp` (`KismetMathLibrary.MakeTransform` (`self.StartFlashlightLocation`) (`self.StartFlashlightRotation`) _relativescale3d) (`KismetMathLibrary.MakeTransform` (`self.EndFlashlightLocation`) (`self.EndFlashlightRotation`) _relativescale3d) _alpha) false false))))

(event `self.Sphere.OnComponentEndOverlap`
  (params (OverlappedComponent :type "PrimitiveComponent Object Reference") (OtherActor :type "Actor Object Reference") (OtherComp :type "PrimitiveComponent Object Reference") (OtherBodyIndex :type Integer))
  (bind _widgetref (`self.WidgetRef`))
  (`|ExecutionSequence`
    (:`then_0`
      (set `self.InCollision` false)
      (set `/Game/Blueprints/Interact/WB_ViewText.Name` "" _widgetref)
      (set `/Game/Blueprints/Interact/WB_ViewText.Name_2` "" _widgetref)
      (`SceneComponent.SetVisibility` (`self.FlashlightRef`) false false))
    (:`then_1`
      (set `self.HoldingDoor` false :!label _label)
      (bind (_direction _alpha) (`Timeline|T_OpenDoor` :!via `Reverse` :!label _label_2)
        (:`Update`
          (`SceneComponent.K2_SetRelativeRotation` (`self.Door`) (`KismetMathLibrary.MakeRotator` 0.0 0.0 (`KismetMathLibrary.Lerp` (`self.StartDoorRotation`) 0.0 _alpha)) false false))
        (:`Finished`
          (if (== (`SceneComponent.RelativeRotation` (`self.Door`)) (struct) :`ErrorTolerance` 0.001)
            (set `self.IsFinished` true)
            (`KismetSystemLibrary.PrintString` "- Held Completely")
            (bind _returnvalue (`GameplayStatics.GetActorOfClass` "/Game/AI/Enemies/BP_Father.BP_Father_C"))
            (`/Game/AI/Enemies/BP_Father.DoorClosed` _returnvalue)))))
    (:`then_2`
      (`LightComponent.SetIntensity` (`self.LightRef`) 0.0 :!label _label_3))))

(event `EnhancedInput|/Game/FirstPerson/Input/Actions/IA_Interact`
  (params (ActionValue :type Boolean) (ElapsedSeconds :type "Float (double-precision)") (TriggeredSeconds :type "Float (double-precision)") (InputAction :type "InputAction Object Reference" :default "/Game/FirstPerson/Input/Actions/IA_Interact.IA_Interact"))
  (:`Started`
    (if (`self.InCollision`)
      (`|ExecutionSequence`
        (:`then_0`
          (set `self.HoldingDoor` true)
          (goto _label_2))
        (:`then_1`
          (goto _label_3)))))
  (:`Canceled`
    (if (`self.IsFinished`) :!label _label_4
      (`|ExecutionSequence`
        (:`then_0`
          (goto _label))
        (:`then_1`
          (set `self.IsFinished` false)
          (`KismetSystemLibrary.PrintString` "- Let Go")
          (bind _returnvalue (`GameplayStatics.GetActorOfClass` "/Game/AI/Enemies/BP_Father.BP_Father_C"))
          (`/Game/AI/Enemies/BP_Father.DoorOpen` _returnvalue)))
      (else
        (set `self.IsFinished` false)
        (goto _label))))
  (:`Completed`
    (goto _label_4)))

(event `EnhancedInput|/Game/FirstPerson/Input/Actions/IA_FlashLight`
  (params (ActionValue :type Boolean) (ElapsedSeconds :type "Float (double-precision)") (TriggeredSeconds :type "Float (double-precision)") (InputAction :type "InputAction Object Reference" :default "/Game/FirstPerson/Input/Actions/IA_FlashLight.IA_FlashLight"))
  (bind _returnvalue (and (`self.InCollision`) (not (`self.HoldingDoor`))))
  (:`Started`
    (if _returnvalue
      (`GameplayStatics.PlaySound2D` "/Game/SoundEffects/FlashlightClick_Shorter.FlashlightClick_Shorter" 1.0 1.0 0.0 null null)
      (`LightComponent.SetIntensity` (`self.LightRef`) 30000.0 :!label _label_5)))
  (:`Ongoing`
    (if _returnvalue
      (goto _label_5)))
  (:`Canceled`
    (`|ExecutionSequence`
      (:`then_0`
        (goto _label_3))
      (:`then_1`
        (if (>= ElapsedSeconds 0.25)
          (if _returnvalue
            (`GameplayStatics.PlaySound2D` "/Game/SoundEffects/FlashlightClick_Shorter.FlashlightClick_Shorter" 1.0 1.0 0.0 null null)
            (goto _label_3))))))
  (:`Completed`
    (`|ExecutionSequence`
      (:`then_0`
        (goto _label_3))
      (:`then_1`
        (if (>= ElapsedSeconds 0.25)
          (if _returnvalue
            (`GameplayStatics.PlaySound2D` "/Game/SoundEffects/FlashlightClick_Shorter.FlashlightClick_Shorter" 1.0 1.0 0.0 null null)
            (goto _label_3)))))))

(fn `UserConstructionScript`
  (`SceneComponent.K2_SetRelativeRotation` (`self.Door`) (`KismetMathLibrary.MakeRotator` 0.0 0.0 (`self.StartDoorRotation`)) false false))