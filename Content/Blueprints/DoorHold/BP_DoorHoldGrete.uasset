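; Hold-to-close door for a timed threat: while the player is in range, holding Interact swings it shut, and releasing lets it swing back open.
; A music timeline acts as the countdown, driving sound-mix volume and a fade widget's opacity, and rewinds at higher speed while the door is held.
; If the timeline finishes, a capture sound plays and the level reloads.
; Includes an Up-key time skip and unconnected flashlight and father-notification logic.
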(event `Key|Up`
  (params (Key :type "Key Structure"))
  (:`Pressed`
    (`TimelineComponent.SetNewTime` (`self.T_Music`) 40.0)))

(event `Key|Down`
  (params (Key :type "Key Structure")))

(event `self.ReceiveBeginPlay`
  (bind _pfcharref (`self.PFCharRef`))
  (`|ExecutionSequence`
    (:`then_0`
      (bind _returnvalue (`|CreateWidget` "/Game/Blueprints/DoorHold/WB_GreteFade.WB_GreteFade_C"))
      (bind _output_get (set `self.FadeWidgetRef` _returnvalue))
      (`UserWidget.AddToViewport` _output_get 0))
    (:`then_1`
      (bind (_direction _volume _fade _timealpha) (`Timeline|T_Music` :`NewTime` 30.0 :!via `PlayFromStart`)
        (:`Update`
          (`|ExecutionSequence`
            (:`then_0`
              (bind _output_get_2 (set `self.Volume` _volume))
              (`GameplayStatics.SetSoundMixClassOverride` "/Game/Blueprints/DoorHold/MasterSoundMixClass.MasterSoundMixClass" "/Game/Blueprints/DoorHold/Music.Music" _output_get_2 1.0 0.0)
              (`KismetSystemLibrary.PrintString` (`KismetStringLibrary.Conv_DoubleToString` _timealpha)))
            (:`then_1`
              (set `/Game/Blueprints/DoorHold/WB_GreteFade.Opacity` _fade (`self.FadeWidgetRef`)))))
        (:`Finished`
          (`/Engine/EditorBlueprintResources/StandardMacros.DoOnce` false :!label _label
            (:`Completed`
              (`GameplayStatics.SetSoundMixClassOverride` "/Game/Blueprints/DoorHold/MasterSoundMixClass.MasterSoundMixClass" "/Game/Blueprints/DoorHold/Music.Music" 0.5 1.0 0.0)
              (`GameplayStatics.PlaySound2D` "/Game/Blueprints/Dialogue/Replica/Sounds/Captured_Cue.Captured_Cue" 1.0 1.0 0.0 null null)
              (`KismetSystemLibrary.Delay` 1.0)
              (bind _returnvalue_2 (`GameplayStatics.GetCurrentLevelName` true))
              (`GameplayStatics.OpenLevel` (`KismetStringLibrary.Conv_StringToName` _returnvalue_2))
              (goto _label :!via `Reset`))))))
    (:`then_2`
      (`GameplayStatics.SetBaseSoundMix` "/Game/Blueprints/DoorHold/MasterSoundMixClass.MasterSoundMixClass")
      (`GameplayStatics.PlaySound2D` "/Game/SoundEffects/SV_ViolinPiece_Cue.SV_ViolinPiece_Cue" 1.0 1.0 0.0 null null))
    (:`then_3`
      (bind _asbp_first_person_character (cast `/Game/FirstPerson/Blueprints/BP_FirstPersonCharacter` (`GameplayStatics.GetPlayerCharacter` 0)))
      (set `self.PFCharRef` _asbp_first_person_character)
      (bind _returnvalue_3 (`|CreateWidget` "/Game/Blueprints/Interact/WB_ViewText.WB_ViewText_C"))
      (bind _output_get_3 (set `self.WidgetRef` _returnvalue_3))
      (`UserWidget.AddToViewport` _output_get_3 0)
      (`self.EnableInput` (`GameplayStatics.GetPlayerController` 0))
      (set `self.FlashlightRef` (`/Game/FirstPerson/Blueprints/BP_FirstPersonCharacter.FlashlightBetter` _pfcharref))
      (set `self.LightRef` (`/Game/FirstPerson/Blueprints/BP_FirstPersonCharacter.SpotLight` _pfcharref)))))

(event `self.Sphere.OnComponentBeginOverlap`
  (params (OverlappedComponent :type "PrimitiveComponent Object Reference") (OtherActor :type "Actor Object Reference") (OtherComp :type "PrimitiveComponent Object Reference") (OtherBodyIndex :type Integer) (bFromSweep :type Boolean) (SweepResult :type "HitResult Structure (by ref)"))
  (if (== OtherActor (`GameplayStatics.GetPlayerCharacter` 0))
    (set `self.InCollision` true)
    (set `/Game/Blueprints/Interact/WB_ViewText.Name` "Hold E to close door" (`self.WidgetRef`))))

(event `self.Sphere.OnComponentEndOverlap`
  (params (OverlappedComponent :type "PrimitiveComponent Object Reference") (OtherActor :type "Actor Object Reference") (OtherComp :type "PrimitiveComponent Object Reference") (OtherBodyIndex :type Integer))
  (bind _t_music (`self.T_Music`))
  (if (`self.IsFinished`)
    (`|ExecutionSequence`
      (:`then_0`
        (if (== OtherActor (`GameplayStatics.GetPlayerCharacter` 0)) :!label _label_2
          (`|ExecutionSequence`
            (:`then_0`
              (set `self.InCollision` false)
              (set `/Game/Blueprints/Interact/WB_ViewText.Name` "" (`self.WidgetRef`)))
            (:`then_1`
              (set `self.HoldingDoor` false :!label _label_3)
              (`TimelineComponent.SetPlayRate` _t_music 1.0)
              (`TimelineComponent.Play` _t_music)
              (bind (_direction _alpha) (`Timeline|T_OpenDoor` :!via `Reverse` :!label _label_4)
                (:`Update`
                  (`SceneComponent.K2_SetRelativeRotation` (`self.Door`) (`KismetMathLibrary.MakeRotator` 0.0 0.0 (`KismetMathLibrary.Lerp` (`self.StartDoorRotation`) 0.0 _alpha)) false false))
                (:`Finished`
                  (if (== (`SceneComponent.RelativeRotation` (`self.Door`)) (struct) :`ErrorTolerance` 0.001)
                    (set `self.IsFinished` true))))))))
      (:`then_1`
        (set `self.IsFinished` false :!label _label_5)))
    (else
      (goto _label_2))))

(event `EnhancedInput|/Game/FirstPerson/Input/Actions/IA_Interact`
  (params (ActionValue :type Boolean) (ElapsedSeconds :type "Float (double-precision)") (TriggeredSeconds :type "Float (double-precision)") (InputAction :type "InputAction Object Reference" :default "/Game/FirstPerson/Input/Actions/IA_Interact.IA_Interact"))
  (bind _t_music (`self.T_Music`))
  (:`Started`
    (if (`self.InCollision`)
      (`|ExecutionSequence`
        (:`then_0`
          (set `self.HoldingDoor` true)
          (`TimelineComponent.SetPlayRate` _t_music 4.0)
          (`TimelineComponent.Reverse` _t_music)
          (if (<= (`self.Volume`) 0.01)
            (`TimelineComponent.SetNewTime` _t_music 0.0)
            (goto _label_4)
            (else
              (goto _label_4)))))))
  (:`Canceled`
    (if (`self.IsFinished`) :!label _label_6
      (`|ExecutionSequence`
        (:`then_0`
          (goto _label_3))
        (:`then_1`
          (goto _label_5)))
      (else
        (goto _label_3))))
  (:`Completed`
    (goto _label_6)))

(fn `UserConstructionScript`
  (`SceneComponent.K2_SetRelativeRotation` (`self.Door`) (`KismetMathLibrary.MakeRotator` 0.0 0.0 (`self.StartDoorRotation`)) false false))