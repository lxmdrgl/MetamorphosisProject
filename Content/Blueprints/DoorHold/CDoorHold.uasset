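; Door actor that the player holds closed by keeping the interact input pressed while standing inside its trigger box.
; Box overlap and Enhanced Input events track presence and held input, so entering with the input already held also closes it.
; A timeline lerps the door's relative rotation from an angled open pose, playing to close and reversing when input is released or the player leaves.
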(event `self.ReceiveBeginPlay`
  (`self.EnableInput` (`GameplayStatics.GetPlayerController` 0)))

(event `self.Box.OnComponentBeginOverlap`
  (params (OverlappedComponent :type "PrimitiveComponent Object Reference") (OtherActor :type "Actor Object Reference") (OtherComp :type "PrimitiveComponent Object Reference") (OtherBodyIndex :type Integer) (bFromSweep :type Boolean) (SweepResult :type "HitResult Structure (by ref)"))
  ;[1 0.2235 0] Overlap
  (if (== OtherActor (`GameplayStatics.GetPlayerCharacter` 0))
    (set `self.doorCollision` true)
    (if (`self.inputHeld`)
      (`self.DoorClose`))))

(event `self.Box.OnComponentEndOverlap`
  (params (OverlappedComponent :type "PrimitiveComponent Object Reference") (OtherActor :type "Actor Object Reference") (OtherComp :type "PrimitiveComponent Object Reference") (OtherBodyIndex :type Integer))
  ;[1 0.2235 0] Overlap
  (if (== OtherActor (`GameplayStatics.GetPlayerCharacter` 0))
    (set `self.doorCollision` false)
    (`self.DoorOpen`)))

(event `EnhancedInput|/Game/FirstPerson/Input/Actions/IA_Interact`
  (params (ActionValue :type Boolean) (ElapsedSeconds :type "Float (double-precision)") (TriggeredSeconds :type "Float (double-precision)") (InputAction :type "InputAction Object Reference" :default "/Game/FirstPerson/Input/Actions/IA_Interact.IA_Interact"))
  ;[1 0.9176 0] Close Door
  (:`Started`
    (set `self.inputHeld` true)
    (if (`self.doorCollision`)
      (`self.DoorClose`)
      (set `self.doorStatus` true)))
  (:`Completed`
    (set `self.inputHeld` false)
    (`self.DoorOpen`)
    (set `self.doorStatus` false)))

(event `DoorClose`
  ;[1 0 0] Door Animation
  (bind (_direction _dooralpha) (`Timeline|DoorAnimationTimeline` :!label _label)
    (:`Update`
      (`SceneComponent.K2_SetRelativeRotation` (`self.Door`) (`KismetMathLibrary.RLerp` (struct :`Yaw` -50.0) (struct) _dooralpha) false false))))

(event `DoorOpen`
  ;[1 0 0] Door Animation
  (goto _label :!via `Reverse`))

(fn `UserConstructionScript`)