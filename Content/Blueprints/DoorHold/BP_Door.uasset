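; BP_Door is an interactable door that toggles open and closed with a rotation animation.
; Each Interact disables CanInteract and flip-flops the T_Door timeline between play and reverse, lerping the Door component's relative rotation to 90 degrees of yaw.
; When the timeline finishes, interaction is re-enabled and ItemName switches between StartName and EndName to match the door's state.
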(event `self.ReceiveBeginPlay`
  (set `self.ItemName` (`self.StartName`)))

(event `/Game/Blueprints/Interact/Interface_Interact.Interact`
  (set `self.CanInteract` false)
  (bind _isa (`/Engine/EditorBlueprintResources/StandardMacros.FlipFlop`)
    (:`A`
      (bind (_direction _alpha) (`Timeline|T_Door` :!label _label)
        (:`Update`
          (set `self.Is A` _isa)
          (`SceneComponent.K2_SetRelativeRotation` (`self.Door`) (`KismetMathLibrary.RLerp` (struct) (struct :`Yaw` 90.0) _alpha) false false))
        (:`Finished`
          (set `self.CanInteract` true)
          (if (`self.Is A`)
            (set `self.ItemName` (`self.EndName`))
            (else
              (set `self.ItemName` (`self.StartName`)))))))
    (:`B`
      (goto _label :!via `Reverse`))))

(fn `UserConstructionScript`)