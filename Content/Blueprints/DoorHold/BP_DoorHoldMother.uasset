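; Door the player holds shut with Interact to repel BP_Mother, with an on-screen prompt inside its trigger sphere.
; Holding plays a timeline that swings it closed and cuts the flashlight beam; releasing or leaving reverses it, notifying Mother of completed closes and reopenings.
; Tick raises Mother's door sound-class volume while the player is in range, and DisableDoor blocks interaction and drops the mesh.
; Most flashlight logic is disconnected.
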(event `self.ReceiveBeginPlay`
  (bind _pfcharref (`self.PFCharRef`))
  (bind _asbp_first_person_character (cast `/Game/FirstPerson/Blueprints/BP_FirstPersonCharacter` (`GameplayStatics.GetPlayerCharacter` 0)))
  (set `self.PFCharRef` _asbp_first_person_character)
  (bind _returnvalue (`|CreateWidget` "/Game/Blueprints/Interact/WB_ViewText.WB_ViewText_C"))
  (bind _output_get (set `self.WidgetRef` _returnvalue))
  (`UserWidget.AddToViewport` _output_get 0)
  (`self.EnableInput` (`GameplayStatics.GetPlayerController` 0))
  (set `self.FlashlightRef` (`/Game/FirstPerson/Blueprints/BP_FirstPersonCharacter.FlashlightBetter` _pfcharref))
  (set `self.LightRef` (`/Game/FirstPerson/Blueprints/BP_FirstPersonCharacter.SpotLight` _pfcharref)))

(event `self.Sphere.OnComponentBeginOverlap`
  (params (OverlappedComponent :type "PrimitiveComponent Object Reference") (OtherActor :type "Actor Object Reference") (OtherComp :type "PrimitiveComponent Object Reference") (OtherBodyIndex :type Integer) (bFromSweep :type Boolean) (SweepResult :type "HitResult Structure (by ref)"))
  (if (== OtherActor (`GameplayStatics.GetPlayerCharacter` 0))
    (set `self.InCollision` true)
    (set `/Game/Blueprints/Interact/WB_ViewText.Name` "Hold E to close door and repel Mother" (`self.WidgetRef`))))

(event `self.Sphere.OnComponentEndOverlap`
  (params (OverlappedComponent :type "PrimitiveComponent Object Reference") (OtherActor :type "Actor Object Reference") (OtherComp :type "PrimitiveComponent Object Reference") (OtherBodyIndex :type Integer))
  (if (`self.IsFinished`)
    (`|ExecutionSequence`
      (:`then_0`
        (if (== OtherActor (`GameplayStatics.GetPlayerCharacter` 0)) :!label _label
          (`|ExecutionSequence`
            (:`then_0`
              (set `self.InCollision` false)
              (set `/Game/Blueprints/Interact/WB_ViewText.Name` "" (`self.WidgetRef`)))
            (:`then_1`
              (set `self.HoldingDoor` false :!label _label_2)
              (bind (_direction _alpha) (`Timeline|T_OpenDoor` :!via `Reverse` :!label _label_3)
                (:`Update`
                  (`SceneComponent.K2_SetRelativeRotation` (`self.Door`) (`KismetMathLibrary.MakeRotator` 0.0 0.0 (`KismetMathLibrary.Lerp` (`self.StartDoorRotation`) 0.0 _alpha)) false false))
                (:`Finished`
                  (if (== (`SceneComponent.RelativeRotation` (`self.Door`)) (struct) :`ErrorTolerance` 0.001)
                    (set `self.IsFinished` true)
                    (bind _returnvalue (`GameplayStatics.GetActorOfClass` "/Game/AI/Enemies/BP_Mother.BP_Mother_C"))
                    (`/Game/AI/Enemies/BP_Mother.DoorClosed` _returnvalue))))))))
      (:`then_1`
        (set `self.IsFinished` false :!label _label_4)
        (bind _returnvalue_2 (`GameplayStatics.GetActorOfClass` "/Game/AI/Enemies/BP_Mother.BP_Mother_C"))
        (`/Game/AI/Enemies/BP_Mother.DoorOpen` _returnvalue_2)))
    (else
      (goto _label))))

(event `EnhancedInput|/Game/FirstPerson/Input/Actions/IA_Interact`
  (params (ActionValue :type Boolean) (ElapsedSeconds :type "Float (double-precision)") (TriggeredSeconds :type "Float (double-precision)") (InputAction :type "InputAction Object Reference" :default "/Game/FirstPerson/Input/Actions/IA_Interact.IA_Interact"))
  (:`Started`
    (if (`self.IsEnabled`)
      (if (`self.InCollision`)
        (`|ExecutionSequence`
          (:`then_0`
            (set `self.HoldingDoor` true)
            (goto _label_3))
          (:`then_1`
            (`LightComponent.SetIntensity` (`self.LightRef`) 0.0))))))
  (:`Canceled`
    (if (`self.IsEnabled`) :!label _label_5
      (if (`self.IsFinished`)
        (`|ExecutionSequence`
          (:`then_0`
            (goto _label_2))
          (:`then_1`
            (goto _label_4)))
        (else
          (goto _label_2)))))
  (:`Completed`
    (goto _label_5)))

(event `EnhancedInput|/Game/FirstPerson/Input/Actions/IA_FlashLight`
  (params (ActionValue :type Boolean) (ElapsedSeconds :type "Float (double-precision)") (TriggeredSeconds :type "Float (double-precision)") (InputAction :type "InputAction Object Reference" :default "/Game/FirstPerson/Input/Actions/IA_FlashLight.IA_FlashLight")))

(event `Disable Door`
  (bind _door (`self.Door`))
  (bind (_relativelocation_x _relativelocation_y _relativelocation_z) (`KismetMathLibrary.BreakVector` (`SceneComponent.RelativeLocation` _door)))
  (set `self.IsEnabled` false)
  (`SceneComponent.K2_SetRelativeLocation` _door (`KismetMathLibrary.MakeVector` _relativelocation_x _relativelocation_y (- _relativelocation_z 300.0)) false false))

(event `self.ReceiveTick`
  (params (DeltaSeconds :type "Float (single-precision)"))
  (`GameplayStatics.SetSoundMixClassOverride` "/Game/Blueprints/DoorHold/MasterSoundMixClass.MasterSoundMixClass" "/Game/Blueprints/DoorHold/MotherDoorSFX.MotherDoorSFX" (`KismetMathLibrary.SelectFloat` 0.2 0.01 (`self.InCollision`)) 1.0 0.0))

(fn `UserConstructionScript`
  (`SceneComponent.K2_SetRelativeRotation` (`self.Door`) (`KismetMathLibrary.MakeRotator` 0.0 0.0 (`self.StartDoorRotation`)) false false))