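; Interactable safe that opens when the player types the correct three-digit code.
; Interact locks player movement and look, blends the camera to the safe, enables its key input and shows a text widget.
; Digit keys append to a string while three point lights show progress, then turn green or red.
; A match swings the door open via timeline and blocks further interaction; a mismatch resets the code, and both exit the view.
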(event `self.ReceiveBeginPlay`
  ;[1 1 1] View safe
  (set `self.UsesMesh` true)
  (bind _asbp_first_person_character (cast `/Game/FirstPerson/Blueprints/BP_FirstPersonCharacter` (`GameplayStatics.GetPlayerCharacter` 0)))
  (set `self.FPCharRef` _asbp_first_person_character)
  (set `self.InteractName` (`self.StartName`))
  (set `self.CanInteract` true)
  (`self.DisableInput` (`GameplayStatics.GetPlayerController` 0))
  (`SceneComponent.SetVisibility` (`self.PointLight1`) false false)
  (`SceneComponent.SetVisibility` (`self.PointLight2`) false false)
  (`SceneComponent.SetVisibility` (`self.PointLight3`) false false))

(event `self.Interact`
  (params (SMRef :type "StaticMeshComponent Object Reference"))
  (bind _returnvalue (`GameplayStatics.GetPlayerController` 0))
  (bind _returnvalue_2 (`GameplayStatics.GetPlayerController` 0))
  ;[1 1 1] View safe
  (if (not (`self.InteractOver`))
    (`CharacterMovementComponent.DisableMovement` (`Character.CharacterMovement` (`self.FPCharRef`)))
    (set `self.CanInteract` false)
    (`Controller.SetIgnoreLookInput` _returnvalue true)
    (`PlayerController.SetViewTargetWithBlend` _returnvalue self 0.5 "VTBlend_Linear" 0.0 false)
    (`KismetSystemLibrary.Delay` 0.5)
    (`self.EnableInput` _returnvalue_2)
    (set `PlayerController.bShowMouseCursor` true _returnvalue_2)
    (bind _returnvalue_3 (`|CreateWidget` "/Game/Blueprints/Interact/WB_ViewText.WB_ViewText_C" _returnvalue_2))
    (bind _output_get (set `self.WidgetRef` _returnvalue_3))
    (`UserWidget.AddToViewport` _output_get 0)
    (set `/Game/Blueprints/Interact/WB_ViewText.Name` (`self.EndName`) (`self.WidgetRef`))))

(event `Exit View`
  (bind _returnvalue (`GameplayStatics.GetPlayerController` 0))
  (bind _returnvalue_2 (`GameplayStatics.GetPlayerController` 0))
  ;[1 1 1] View safe
  (`Widget.RemoveFromParent` (`self.WidgetRef`))
  (set `PlayerController.bShowMouseCursor` false _returnvalue_2)
  (`PlayerController.SetViewTargetWithBlend` _returnvalue_2 (`self.FPCharRef`) 0.5 "VTBlend_Linear" 0.0 false)
  (`KismetSystemLibrary.Delay` 0.5)
  (`self.DisableInput` _returnvalue)
  (set `self.CanInteract` true)
  (`Controller.SetIgnoreLookInput` _returnvalue false)
  (`CharacterMovementComponent.SetMovementMode` (`Character.CharacterMovement` (`self.FPCharRef`)) "MOVE_Walking" 0))

(event `Open Door`
  ;[1 1 1] Open door / inputs
  (set `self.InteractOver` true)
  (bind (_direction _alpha) (`Timeline|T_OpenDoor`)
    (:`Update`
      (`SceneComponent.K2_SetRelativeRotation` (`self.SafeDoor`) (`KismetMathLibrary.MakeRotator` 0.0 0.0 (`KismetMathLibrary.Lerp` 0.0 -150.0 _alpha)) false false)
      (`self.Exit View`))))

(event `Try Code`
  ;[1 1 1] Try Code
  (if (>= (`KismetStringLibrary.Len` (`self.CurrCode`)) 1)
    (`SceneComponent.SetVisibility` (`self.PointLight1`) true false)
    (if (>= (`KismetStringLibrary.Len` (`self.CurrCode`)) 2)
      (`SceneComponent.SetVisibility` (`self.PointLight2`) true false)
      (if (>= (`KismetStringLibrary.Len` (`self.CurrCode`)) 3)
        (`SceneComponent.SetVisibility` (`self.PointLight3`) true false)
        (if (`KismetStringLibrary.EqualEqual_StrStr` (`self.CurrCode`) (`self.Code`))
          (`LightComponent.SetLightColor` (`self.PointLight1`) (`self.Green`) true)
          (`LightComponent.SetLightColor` (`self.PointLight2`) (`self.Green`) true)
          (`LightComponent.SetLightColor` (`self.PointLight3`) (`self.Green`) true)
          (`self.DisableInput` (`GameplayStatics.GetPlayerController` 0))
          (`KismetSystemLibrary.Delay` 0.5)
          (`self.Open Door`)
          (else
            (`LightComponent.SetLightColor` (`self.PointLight1`) (`self.Red`) true)
            (`LightComponent.SetLightColor` (`self.PointLight2`) (`self.Red`) true)
            (`LightComponent.SetLightColor` (`self.PointLight3`) (`self.Red`) true)
            (set `self.CurrCode` "")
            (`KismetSystemLibrary.Delay` 0.5)
            (`SceneComponent.SetVisibility` (`self.PointLight1`) false false)
            (`SceneComponent.SetVisibility` (`self.PointLight2`) false false)
            (`SceneComponent.SetVisibility` (`self.PointLight3`) false false)
            (`LightComponent.SetLightColor` (`self.PointLight1`) (`self.White`) true)
            (`LightComponent.SetLightColor` (`self.PointLight2`) (`self.White`) true)
            (`LightComponent.SetLightColor` (`self.PointLight3`) (`self.White`) true)
            (`self.Exit View`)))))))

(event `Key|Zero`
  (params (Key :type "Key Structure"))
  ;[1 1 1] Numpad keys
  (:`Pressed`
    (set `self.CurrCode` (`KismetStringLibrary.Concat_StrStr` (`self.CurrCode`) "0"))
    (`self.Try Code`)))

(event `Key|One`
  (params (Key :type "Key Structure"))
  ;[1 1 1] Numpad keys
  (:`Pressed`
    (set `self.CurrCode` (`KismetStringLibrary.Concat_StrStr` (`self.CurrCode`) "1"))
    (`self.Try Code`)))

(event `Key|Two`
  (params (Key :type "Key Structure"))
  ;[1 1 1] Numpad keys
  (:`Pressed`
    (set `self.CurrCode` (`KismetStringLibrary.Concat_StrStr` (`self.CurrCode`) "2"))
    (`self.Try Code`)))

(event `Key|Three`
  (params (Key :type "Key Structure"))
  ;[1 1 1] Numpad keys
  (:`Pressed`
    (set `self.CurrCode` (`KismetStringLibrary.Concat_StrStr` (`self.CurrCode`) "3"))
    (`self.Try Code`)))

(event `Key|Four`
  (params (Key :type "Key Structure"))
  ;[1 1 1] Numpad keys
  (:`Pressed`
    (set `self.CurrCode` (`KismetStringLibrary.Concat_StrStr` (`self.CurrCode`) "4"))
    (`self.Try Code`)))

(event `Key|Five`
  (params (Key :type "Key Structure"))
  ;[1 1 1] Numpad keys
  (:`Pressed`
    (set `self.CurrCode` (`KismetStringLibrary.Concat_StrStr` (`self.CurrCode`) "5"))
    (`self.Try Code`)))

(event `Key|Six`
  (params (Key :type "Key Structure"))
  ;[1 1 1] Numpad keys
  (:`Pressed`
    (set `self.CurrCode` (`KismetStringLibrary.Concat_StrStr` (`self.CurrCode`) "6"))
    (`self.Try Code`)))

(event `Key|Seven`
  (params (Key :type "Key Structure"))
  ;[1 1 1] Numpad keys
  (:`Pressed`
    (set `self.CurrCode` (`KismetStringLibrary.Concat_StrStr` (`self.CurrCode`) "7"))
    (`self.Try Code`)))

(event `Key|Eight`
  (params (Key :type "Key Structure"))
  ;[1 1 1] Numpad keys
  (:`Pressed`
    (set `self.CurrCode` (`KismetStringLibrary.Concat_StrStr` (`self.CurrCode`) "8"))
    (`self.Try Code`)))

(event `Key|Nine`
  (params (Key :type "Key Structure"))
  ;[1 1 1] Numpad keys
  (:`Pressed`
    (set `self.CurrCode` (`KismetStringLibrary.Concat_StrStr` (`self.CurrCode`) "9"))
    (`self.Try Code`)))

(fn `Get Name`
  (returns (GetName :type Text))
  (return ""))

(fn `UserConstructionScript`)