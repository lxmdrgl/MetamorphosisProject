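; BP_Window is an interactable window that slides open once the player has a key and its barricade is cleared.
; Every tick it counts all BP_Plank actors in the level, treats itself as unbarricaded only when exactly two exist, and sets the prompt override for locked or barricaded states.
; Interact checks both conditions, then plays a timeline that lerps the Down component's relative location.
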(event `self.ReceiveBeginPlay`
  (bind _asbp_first_person_character (cast `/Game/FirstPerson/Blueprints/BP_FirstPersonCharacter` (`GameplayStatics.GetPlayerCharacter` 0)))
  (set `self.FPCharRef` _asbp_first_person_character)
  (set `self.InteractName` "unlock window"))

(event `/Game/Blueprints/Interact/Interface_Interact.Interact`
  (params (SMRef :type "StaticMeshComponent Object Reference"))
  (if (`self.IsBarricaded`)
    _
    (elif (`/Game/FirstPerson/Blueprints/BP_FirstPersonCharacter.IsKeyEnabled` (`self.FPCharRef`))
      (set `self.InteractOver` true)
      (bind (_direction _alpha) (`Timeline|T_WindowOpen` :!via `PlayFromStart`)
        (:`Update`
          (`SceneComponent.K2_SetRelativeLocation` (`self.Down`) (`KismetMathLibrary.VLerp` (`self.StartLocation`) (`self.EndLocation`) _alpha) false false))))))

(event `self.ReceiveTick`
  (params (DeltaSeconds :type "Float (single-precision)"))
  (bind _outactors (`GameplayStatics.GetAllActorsOfClass` "/Game/Blueprints/Level2PuzzleItems/Plank/BP_Plank.BP_Plank_C"))
  (if (== (`KismetArrayLibrary.Array_Length` _outactors) 2)
    (set `self.IsBarricaded` false)
    (else
      (set `self.IsBarricaded` true)))
  (if (`/Game/FirstPerson/Blueprints/BP_FirstPersonCharacter.IsKeyEnabled` (`self.FPCharRef`))
    (if (`self.IsBarricaded`)
      (set `self.NameOveride` "Window is barricaded")
      (else
        (set `self.NameOveride` "")))
    (else
      (set `self.NameOveride` "Window is locked"))))

(fn `UserConstructionScript`)