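; Gregor's desk in the second room, scripting a dialogue sequence around the player's flashlight and drawer interaction.
; On BeginPlay it disables player interaction and plays scene 5 through BP_Dialogue; EndScene6 then grants the flashlight and re-enables interaction.
; Tick polls all BP_Desk3_Drawer actors and, shortly after one opens, plays scene 6 once.
; EndScene7 disables interaction again; event names and debug prints number scenes one above the PlayScene indices.
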(event `self.ReceiveBeginPlay`
  (`KismetSystemLibrary.Delay` 0.05)
  (bind _asbp_first_person_character (cast `/Game/FirstPerson/Blueprints/BP_FirstPersonCharacter` (`GameplayStatics.GetPlayerCharacter` 0)))
  (bind _output_get (set `self.FPCharRef` _asbp_first_person_character))
  (set `/Game/FirstPerson/Blueprints/BP_FirstPersonCharacter.InteractEnabled` false _output_get)
  (bind _returnvalue (`GameplayStatics.GetActorOfClass` "/Game/Blueprints/Dialogue/BP_Dialogue.BP_Dialogue_C"))
  (`/Game/Blueprints/Dialogue/BP_Dialogue.PlayScene` _returnvalue 5)
  (`KismetSystemLibrary.PrintString` "play 6"))

(event `EndScene6`
  (`/Game/FirstPerson/Blueprints/BP_FirstPersonCharacter.FlashlightPickedUp` (`self.FPCharRef`))
  (set `/Game/FirstPerson/Blueprints/BP_FirstPersonCharacter.InteractEnabled` true (`self.FPCharRef`)))

(event `self.ReceiveTick`
  (params (DeltaSeconds :type "Float (single-precision)"))
  (bind _outactors (`GameplayStatics.GetAllActorsOfClass` "/Game/Blueprints/Second_Room/Desk/BP_Desk3_Drawer.BP_Desk3_Drawer_C"))
  (for _array_element _outactors
    (if (`/Game/Blueprints/Second_Room/Desk/BP_Desk3_Drawer.IsOpened` _array_element)
      (`KismetSystemLibrary.Delay` 0.5)
      (`/Engine/EditorBlueprintResources/StandardMacros.DoOnce` false
        (:`Completed`
          (bind _returnvalue (`GameplayStatics.GetActorOfClass` "/Game/Blueprints/Dialogue/BP_Dialogue.BP_Dialogue_C"))
          (`/Game/Blueprints/Dialogue/BP_Dialogue.PlayScene` _returnvalue 6)
          (`KismetSystemLibrary.PrintString` "play 7"))))))

(event `EndScene7`
  (set `/Game/FirstPerson/Blueprints/BP_FirstPersonCharacter.InteractEnabled` false (`self.FPCharRef`)))

(fn `UserConstructionScript`)