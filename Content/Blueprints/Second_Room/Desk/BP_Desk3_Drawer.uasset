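; Interactable desk drawer in the Second_Room folder that slides open and closed.
; Interact compares the drawer's relative location to its start position, then plays the open timeline forward or in reverse.
; The timeline lerps the drawer between start and end locations at a play rate raised on BeginPlay.
; CanInteract is cleared when movement begins and restored when the timeline finishes, blocking re-triggering mid-slide.
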(event `self.ReceiveBeginPlay`
  (set `self.InteractName` "interact with drawer")
  (`TimelineComponent.SetPlayRate` (`self.T_OpenDrawer`) 2.0))

(event `/Game/Blueprints/Interact/Interface_Interact.Interact`
  (params (SMRef :type "StaticMeshComponent Object Reference"))
  (set `self.CanInteract` false)
  (if (== (`SceneComponent.RelativeLocation` (`self.Drawer`)) (`self.StartLocation`) :`ErrorTolerance` 0.001)
    (bind (_direction _alpha) (`Timeline|T_OpenDrawer` :!via `PlayFromStart` :!label _label)
      (:`Update`
        (`SceneComponent.K2_SetRelativeLocation` (`self.Drawer`) (`KismetMathLibrary.VLerp` (`self.StartLocation`) (`self.EndLocation`) _alpha) false false))
      (:`Finished`
        (set `self.CanInteract` true)))
    (else
      (goto _label :!via `ReverseFromEnd`))))

(fn `UserConstructionScript`)