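; BP_DeskLight is an interactable desk lamp that toggles its light when the player interacts with it.
; BeginPlay sets the interaction prompt and, if StartOn is false, fires the shared FlipFlop once to start it dark.
; Interact drives the same FlipFlop, switching SpotLight visibility and propagating it to child components.
; The construction script applies LightColor to both SpotLight and PointLight.
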(event `self.ReceiveBeginPlay`
  (bind _spotlight (`self.SpotLight`))
  (set `self.InteractName` "interact with desk light")
  (if (not (`self.StartOn`))
    (`/Engine/EditorBlueprintResources/StandardMacros.FlipFlop` :!label _label
      (:`A`
        (`SceneComponent.SetVisibility` _spotlight false true))
      (:`B`
        (`SceneComponent.SetVisibility` _spotlight true true)))))

(event `/Game/Blueprints/Interact/Interface_Interact.Interact`
  (params (SMRef :type "StaticMeshComponent Object Reference"))
  (goto _label))

(fn `UserConstructionScript`
  (`LightComponent.SetLightColor` (`self.SpotLight`) (`self.LightColor`) true)
  (`LightComponent.SetLightColor` (`self.PointLight`) (`self.LightColor`) true))