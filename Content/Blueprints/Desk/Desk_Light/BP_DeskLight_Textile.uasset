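; Interactable desk light that changes what appears on the desk each time it is switched back on.
; Interact drives a FlipFlop toggling the SpotLight, while OnCount shows FolderHolder, then Typewriter, then Textile on successive switch-ons, hiding the first two again at switch-off.
; The third switch-on also makes BP_TextilePickup_3 interactable.
; BeginPlay either disables prop collision (StartOn) or runs the first toggle; construction applies LightColor.
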(event `self.ReceiveBeginPlay`
  (bind _spotlight (`self.SpotLight`))
  (set `self.InteractName` "interact with desk light")
  (if (`self.StartOn`)
    (`PrimitiveComponent.SetCollisionEnabled` (`self.Typewriter`) "NoCollision")
    (`PrimitiveComponent.SetCollisionEnabled` (`self.FolderHolder`) "NoCollision")
    (else
      (`/Engine/EditorBlueprintResources/StandardMacros.FlipFlop` :!label _label
        (:`A`
          (`SceneComponent.SetVisibility` _spotlight false true)
          (`|ExecutionSequence`
            (:`then_0`
              (if (== (`self.OnCount`) 1)
                (`SceneComponent.SetVisibility` (`self.FolderHolder`) false false)))
            (:`then_1`
              (if (== (`self.OnCount`) 2)
                (`SceneComponent.SetVisibility` (`self.Typewriter`) false false)))))
        (:`B`
          (`SceneComponent.SetVisibility` _spotlight true true)
          (`/Engine/EditorBlueprintResources/StandardMacros.IncrementInt` (`self.OnCount`)
            (:`  `
              (`|ExecutionSequence`
                (:`then_0`
                  (if (== (`self.OnCount`) 1)
                    (`SceneComponent.SetVisibility` (`self.FolderHolder`) true false)))
                (:`then_1`
                  (if (== (`self.OnCount`) 2)
                    (`SceneComponent.SetVisibility` (`self.Typewriter`) true false)))
                (:`then_2`
                  (if (== (`self.OnCount`) 3)
                    (`SceneComponent.SetVisibility` (`self.Textile`) true false)
                    (bind _returnvalue (`GameplayStatics.GetActorOfClass` "/Game/Blueprints/Textiles/BP_TextilePickup_3.BP_TextilePickup_3_C"))
                    (set `/Game/Blueprints/Interact/BP_Item.CanInteract` true _returnvalue)))))))))))

(event `/Game/Blueprints/Interact/Interface_Interact.Interact`
  (params (SMRef :type "StaticMeshComponent Object Reference"))
  (goto _label))

(fn `UserConstructionScript`
  (`LightComponent.SetLightColor` (`self.SpotLight`) (`self.LightColor`) true)
  (`LightComponent.SetLightColor` (`self.PointLight`) (`self.LightColor`) true))