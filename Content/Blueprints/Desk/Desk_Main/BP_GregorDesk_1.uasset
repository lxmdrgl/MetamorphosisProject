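; Gregor's interactable desk, whose middle and top drawers slide open and shut, and which can drive the game's opening sequence.
; With PlayOpening set, it fades in, freezes the player and starts the first dialogue scene, restoring control when that ends.
; Interact toggles the chosen drawer through timeline lerps, and opening all three triggers another BP_Dialogue scene.
; A blocking volume is removed by EndScene2, or at start when the opening is skipped.
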(event `self.ReceiveBeginPlay`
  (bind _fpcharref (`self.FPCharRef`))
  (bind _asbp_first_person_character (cast `/Game/FirstPerson/Blueprints/BP_FirstPersonCharacter` (`GameplayStatics.GetPlayerCharacter` 0)))
  (set `self.FPCharRef` _asbp_first_person_character)
  (set `self.InteractName` "interact with")
  (set `self.UsesMesh` true)
  (`TimelineComponent.SetPlayRate` (`self.Timeline`) 2.0)
  (`TimelineComponent.SetPlayRate` (`self.OpenDrawer`) 2.0)
  ;[1 1 1] Scenes
  (if (`self.PlayOpening`)
    (`|ExecutionSequence`
      (:`then_0`
        (bind _returnvalue (`|CreateWidget` "/Game/Blueprints/Interact/WB_Fade.WB_Fade_C"))
        (`UserWidget.AddToViewport` _returnvalue 0)
        (`KismetSystemLibrary.Delay` 0.5)
        (`UserWidget.PlayAnimation` _returnvalue (`/Game/Blueprints/Interact/WB_Fade.FadeOut` _returnvalue) 0.0 1 "Forward" 0.15 false))
      (:`then_1`
        (set `self.CanInteract` false)
        (`CharacterMovementComponent.DisableMovement` (`Character.CharacterMovement` _fpcharref))
        (set `/Game/FirstPerson/Blueprints/BP_FirstPersonCharacter.InteractEnabled` false _fpcharref)
        (`KismetSystemLibrary.Delay` 2.0)
        (`self.PlayScene1`))
      (:`then_2`
        (bind _returnvalue_2 (`GameplayStatics.GetActorOfClass` "/Game/Blueprints/Dialogue/BP_Dialogue.BP_Dialogue_C"))
        (bind _output_get (set `self.DialogueRef` _returnvalue_2))
        (add `/Game/Blueprints/Dialogue/BP_Dialogue.EndScene1` _output_get (delegate `EndScene1`))))
    (elif (`KismetSystemLibrary.IsValid` (`self.BlockingVolume`))
      (`self.K2_DestroyActor` (`self.BlockingVolume`)))))

(event `/Game/Blueprints/Interact/Interface_Interact.Interact`
  (params (SMRef :type "StaticMeshComponent Object Reference"))
  (bind _smref (`self.SMRef`))
  (bind _smref_2 (`self.SMRef`))
  (bind _smref_3 (`self.SMRef`))
  (bind _returnvalue (== (`self.SMRef`) (`self.Middle Drawer`)))
  (bind _relativelocation_x (`KismetMathLibrary.BreakVector` (`SceneComponent.RelativeLocation` (`self.SMRef`))))
  (bind (_relativelocation_x_2 _relativelocation_y _relativelocation_z) (`KismetMathLibrary.BreakVector` (`SceneComponent.RelativeLocation` _smref_2)))
  (bind _relativelocation_x_3 (`KismetMathLibrary.BreakVector` (`SceneComponent.RelativeLocation` (`self.SMRef`))))
  (bind (_relativelocation_x_4 _relativelocation_y_2 _relativelocation_z_2) (`KismetMathLibrary.BreakVector` (`SceneComponent.RelativeLocation` _smref_3)))
  (bind _returnvalue_2 (or false (== _smref (`self.Top Left Drawer`)) false (== _smref (`self.Top Right Drawer`))))
  (set `self.SMRef` SMRef)
  (set `self.CanInteract` false)
  (`|ExecutionSequence`
    (:`then_0`
      (if _returnvalue_2
        (if (`KismetMathLibrary.NearlyEqual_FloatFloat` _relativelocation_x (`self.SideStart`))
          (bind (_direction _alpha) (`Timeline|OpenDrawer` :!via `PlayFromStart` :!label _label)
            (:`Update`
              (`SceneComponent.K2_SetRelativeLocation` _smref_2 (`KismetMathLibrary.MakeVector` (`KismetMathLibrary.Lerp` (`self.SideStart`) (`self.SideEnd`) _alpha) _relativelocation_y _relativelocation_z) false false))
            (:`Finished`
              (set `self.CanInteract` true :!label _label_2)))
          (else
            (goto _label :!via `ReverseFromEnd`)))))
    (:`then_1`
      (if _returnvalue
        (if (`KismetMathLibrary.NearlyEqual_FloatFloat` _relativelocation_x_3 (`self.MidStart`))
          (bind (_direction_2 _alpha_2) (`Timeline|Timeline` :!via `PlayFromStart` :!label _label_3)
            (:`Update`
              (`SceneComponent.K2_SetRelativeLocation` _smref_3 (`KismetMathLibrary.MakeVector` (`KismetMathLibrary.Lerp` (`self.MidStart`) (`self.MidEnd`) _alpha_2) _relativelocation_y_2 _relativelocation_z_2) false false))
            (:`Finished`
              (goto _label_2)))
          (else
            (goto _label_3 :!via `ReverseFromEnd`)))))
    (:`then_2`
      (if (and (not _returnvalue_2) (not _returnvalue))
        (goto _label_2)))
    (:`then_3`
      (if (== (`self.SMRef`) (`self.Middle Drawer`))
        (`/Engine/EditorBlueprintResources/StandardMacros.DoOnce` false
          (:`Completed`
            (bind _result (`/Engine/EditorBlueprintResources/StandardMacros.IncrementInt` (`self.OpenCount`) :!label _label_4)
              (:`  `
                (if (== _result 3)
                  (`KismetSystemLibrary.Delay` 0.0)
                  (if (`self.PlayOpening`)
                    (bind _returnvalue_3 (`GameplayStatics.GetActorOfClass` "/Game/Blueprints/Dialogue/BP_Dialogue.BP_Dialogue_C"))
                    (`/Game/Blueprints/Dialogue/BP_Dialogue.PlayScene` _returnvalue_3 1)))))))))
    (:`then_4`
      (if (== (`self.SMRef`) (`self.Bottom Left Drawer`))
        _))
    (:`then_5`
      (if (== (`self.SMRef`) (`self.Top Left Drawer`))
        (`/Engine/EditorBlueprintResources/StandardMacros.DoOnce` false
          (:`Completed`
            (goto _label_4)))))
    (:`then_6`
      (if (== (`self.SMRef`) (`self.Bottom Right Drawer`))
        _))
    (:`then_7`
      (if (== (`self.SMRef`) (`self.Top Right Drawer`))
        (`/Engine/EditorBlueprintResources/StandardMacros.DoOnce` false
          (:`Completed`
            (goto _label_4)))))))

(event `EndScene1`
  ;[1 1 1] Scenes
  (set `self.CanInteract` true)
  (set `/Game/FirstPerson/Blueprints/BP_FirstPersonCharacter.InteractEnabled` true (`self.FPCharRef`))
  (`CharacterMovementComponent.SetMovementMode` (`Character.CharacterMovement` (`self.FPCharRef`)) "MOVE_Walking" 0))

(event `EndScene2`
  (bind _blockingvolume (`self.BlockingVolume`))
  ;[1 1 1] Scenes
  (if (`KismetSystemLibrary.IsValid` _blockingvolume)
    (`self.K2_DestroyActor` _blockingvolume)))

(fn `UserConstructionScript`)