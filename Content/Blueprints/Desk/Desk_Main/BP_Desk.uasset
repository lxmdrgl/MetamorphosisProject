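; BP_Desk is an interactable desk whose top-left, top-right and middle drawers slide open and closed.
; Interact takes the targeted mesh, blocks further interaction, and picks the side or middle drawer macro by component comparison.
; Each macro checks local X against its start position, then plays or reverses a double-speed timeline that lerps the drawer, re-enabling interaction when finished.
; Bottom drawer comparisons exist but are unused.
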(event `self.ReceiveBeginPlay`
  (bind _asbp_first_person_character (cast `/Game/FirstPerson/Blueprints/BP_FirstPersonCharacter` (`GameplayStatics.GetPlayerCharacter` 0)))
  (set `self.FPCharRef` _asbp_first_person_character)
  (set `self.InteractName` "interact with")
  (set `self.UsesMesh` true)
  (`TimelineComponent.SetPlayRate` (`self.Timeline`) 2.0)
  (`TimelineComponent.SetPlayRate` (`self.OpenDrawer`) 2.0))

(event `/Game/Blueprints/Interact/Interface_Interact.Interact`
  (params (SMRef :type "StaticMeshComponent Object Reference"))
  (bind _smref (`self.SMRef`))
  (bind _smref_2 (`self.SMRef`))
  (bind _smref_3 (`self.SMRef`))
  (bind _returnvalue (== (`self.SMRef`) (`self.Middle Drawer`)))
  (bind _relativelocation_x (`KismetMathLibrary.BreakVector` (`SceneComponent.RelativeLocation` (`self.SMRef`))))
  (bind (_relativelocation_x_2 _relativelocation_y _relativelocation_z) (`KismetMathLibrary.BreakVector` (`SceneComponent.RelativeLocation` _smref_2)))
  (bind _relativelocation_x_3 (`KismetMathLibrary.BreakVector` (`SceneComponent.RelativeLocation` (`self.SMRef`))))
  (bind (_relativelocation_x_4 _relativelocation_y_2 _relativelocation_z_2) (`KismetMathLibrary.BreakVector` (`SceneComponent.RelativeLocation` _smref_3)))
  (bind _returnvalue_2 (or false (== _smref (`self.Top Left Drawer`)) false (== _smref (`self.Top Right Drawer`))))
  (set `self.SMRef` SMRef)
  (set `self.CanInteract` false)
  (`|ExecutionSequence`
    (:`then_0`
      (if _returnvalue_2
        (if (`KismetMathLibrary.NearlyEqual_FloatFloat` _relativelocation_x (`self.SideStart`))
          (bind (_direction _alpha) (`Timeline|OpenDrawer` :!via `PlayFromStart` :!label _label)
            (:`Update`
              (`SceneComponent.K2_SetRelativeLocation` _smref_2 (`KismetMathLibrary.MakeVector` (`KismetMathLibrary.Lerp` (`self.SideStart`) (`self.SideEnd`) _alpha) _relativelocation_y _relativelocation_z) false false))
            (:`Finished`
              (set `self.CanInteract` true :!label _label_2)))
          (else
            (goto _label :!via `ReverseFromEnd`)))))
    (:`then_1`
      (if _returnvalue
        (if (`KismetMathLibrary.NearlyEqual_FloatFloat` _relativelocation_x_3 (`self.MidStart`))
          (bind (_direction_2 _alpha_2) (`Timeline|Timeline` :!via `PlayFromStart` :!label _label_3)
            (:`Update`
              (`SceneComponent.K2_SetRelativeLocation` _smref_3 (`KismetMathLibrary.MakeVector` (`KismetMathLibrary.Lerp` (`self.MidStart`) (`self.MidEnd`) _alpha_2) _relativelocation_y_2 _relativelocation_z_2) false false))
            (:`Finished`
              (goto _label_2)))
          (else
            (goto _label_3 :!via `ReverseFromEnd`)))))
    (:`then_2`
      (if (and (not _returnvalue_2) (not _returnvalue))
        (goto _label_2)))))

(fn `UserConstructionScript`)