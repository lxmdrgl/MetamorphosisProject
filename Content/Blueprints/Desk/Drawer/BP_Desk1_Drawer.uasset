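; Interactable desk drawer that slides open and closed along its relative X axis.
; Interact checks whether the drawer sits at SideStart, then plays or reverses a double-speed Timeline lerping it toward SideEnd.
; Interaction stays disabled until the Timeline finishes.
; DoOnce gates set IsOpened on the first opening and, when that motion finishes, call AddOpened on the BP_GregorDesk_1 actor found in the level.
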(event `self.ReceiveBeginPlay`
  (`TimelineComponent.SetPlayRate` (`self.Timeline`) 2.0)
  (set `self.InteractName` "interact with drawer"))

(event `/Game/Blueprints/Interact/Interface_Interact.Interact`
  (params (SMRef :type "StaticMeshComponent Object Reference"))
  (bind _relativelocation_x (`KismetMathLibrary.BreakVector` (`SceneComponent.RelativeLocation` (`self.Drawer`))))
  (bind (_relativelocation_x_2 _relativelocation_y _relativelocation_z) (`KismetMathLibrary.BreakVector` (`SceneComponent.RelativeLocation` (`self.Drawer`))))
  (set `self.CanInteract` false)
  (if (`KismetMathLibrary.NearlyEqual_FloatFloat` _relativelocation_x (`self.SideStart`))
    (`|ExecutionSequence`
      (:`then_0`
        (bind (_direction _alpha) (`Timeline|Timeline` :!label _label)
          (:`Update`
            (`SceneComponent.K2_SetRelativeLocation` (`self.Drawer`) (`KismetMathLibrary.MakeVector` (`KismetMathLibrary.Lerp` (`self.SideStart`) (`self.SideEnd`) _alpha) _relativelocation_y _relativelocation_z) false false))
          (:`Finished`
            (`|ExecutionSequence`
              (:`then_0`
                (set `self.CanInteract` true))
              (:`then_1`
                (`/Engine/EditorBlueprintResources/StandardMacros.DoOnce` false
                  (:`Completed`
                    (bind _returnvalue (`GameplayStatics.GetActorOfClass` "/Game/Blueprints/Desk/Desk_Main/BP_GregorDesk_1.BP_GregorDesk_1_C"))
                    (`/Game/Blueprints/Desk/Desk_Main/BP_GregorDesk_1.AddOpened` _returnvalue))))))))
      (:`then_1`
        (`/Engine/EditorBlueprintResources/StandardMacros.DoOnce` false
          (:`Completed`
            (set `self.IsOpened` true)))))
    (else
      (goto _label :!via `Reverse`))))

(fn `UserConstructionScript`)