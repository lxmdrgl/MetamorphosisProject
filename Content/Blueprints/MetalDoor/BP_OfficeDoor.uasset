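; Interactable office exit door that ends the level once the player has collected textiles, showing a hint prompt until then.
; Interact freezes movement, runs a fade transition, starts a BP_Dialogue scene and spawns BP_ChiefStatic at the door.
; EndScene5 then plays the capture sound and the chief's attack montage, fades again and opens SecondLevel.
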(event `self.ReceiveBeginPlay`
  (bind _asbp_first_person_character (cast `/Game/FirstPerson/Blueprints/BP_FirstPersonCharacter` (`GameplayStatics.GetPlayerCharacter` 0)))
  (set `self.FPCharRef` _asbp_first_person_character)
  (set `self.InteractName` "leave office")
  (bind _returnvalue (`|CreateWidget` "/Game/Blueprints/Interact/WB_Fade.WB_Fade_C"))
  (set `self.FadeWidgetRef` _returnvalue))

(event `self.ReceiveTick`
  (params (DeltaSeconds :type "Float (single-precision)"))
  (if (< (`/Game/FirstPerson/Blueprints/BP_FirstPersonCharacter.TextileCount` (`self.FPCharRef`)) 1)
    (set `self.NameOveride` "You need to find the rest of the textiles before leaving")
    (else
      (set `self.NameOveride` ""))))

(event `/Game/Blueprints/Interact/Interface_Interact.Interact`
  (params (SMRef :type "StaticMeshComponent Object Reference"))
  (bind _fadewidgetref (`self.FadeWidgetRef`))
  (bind _fadewidgetref_2 (`self.FadeWidgetRef`))
  (bind _returnvalue (`SceneComponent.K2_GetComponentToWorld` (`self.Door`)))
  ;[1 1 1] Comment
  (if (not (< (`/Game/FirstPerson/Blueprints/BP_FirstPersonCharacter.TextileCount` (`self.FPCharRef`)) 1))
    (set `self.InteractOver` true)
    (`CharacterMovementComponent.DisableMovement` (`Character.CharacterMovement` (`self.FPCharRef`)))
    (`UserWidget.AddToViewport` (`self.FadeWidgetRef`) 0)
    (`UserWidget.PlayAnimationReverse` _fadewidgetref_2 (`/Game/Blueprints/Interact/WB_Fade.FadeOut` _fadewidgetref_2) 1.0 true)
    (`KismetSystemLibrary.Delay` 1.0)
    (`|ExecutionSequence`
      (:`then_0`
        (`UserWidget.PlayAnimationForward` _fadewidgetref (`/Game/Blueprints/Interact/WB_Fade.FadeOut` _fadewidgetref) 1.0 false)
        (`KismetSystemLibrary.Delay` 0.95)
        (`Widget.RemoveFromParent` (`self.FadeWidgetRef`))
        (bind _returnvalue_2 (`GameplayStatics.GetActorOfClass` "/Game/Blueprints/Dialogue/BP_Dialogue.BP_Dialogue_C"))
        (`/Game/Blueprints/Dialogue/BP_Dialogue.PlayScene` _returnvalue_2 4))
      (:`then_1`
        (bind _returnvalue_3 (`|SpawnActorFromClass` "/Game/Blueprints/Characters/Chief/BP_ChiefStatic.BP_ChiefStatic_C" (`KismetMathLibrary.MakeTransform` (`KismetMathLibrary.MakeVector` (+ (.x (.location _returnvalue)) 0.0) (.y (.location _returnvalue)) (.z (.location _returnvalue)))) "AlwaysSpawn" "OverrideRootScale" null null))
        (set `self.ChiefRef` _returnvalue_3)))))

(event `EndScene5`
  (bind _fadewidgetref (`self.FadeWidgetRef`))
  ;[1 1 1] Comment
  (`GameplayStatics.PlaySound2D` "/Game/Blueprints/Dialogue/Replica/Sounds/Captured_Cue.Captured_Cue" 1.0 1.0 0.0 null null)
  (`Character.PlayAnimMontage` (`self.ChiefRef`) "/Game/AI/BasicAI_2/Animations/Zombie_Attack_Chief_Montage.Zombie_Attack_Chief_Montage" 1.0 "None")
  (`KismetSystemLibrary.Delay` 1.0)
  (`UserWidget.AddToViewport` (`self.FadeWidgetRef`) 0)
  (`UserWidget.PlayAnimationReverse` _fadewidgetref (`/Game/Blueprints/Interact/WB_Fade.FadeOut` _fadewidgetref) 1.0 true)
  (`KismetSystemLibrary.Delay` 1.0)
  (`GameplayStatics.OpenLevel` "SecondLevel"))

(fn `UserConstructionScript`)