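; Base actor for readable paper notes that the player picks up to view on screen and drops with Tab.
; On BeginPlay it creates a note widget, fed the note's material, and a prompt widget for the drop key.
; Interact hides the mesh, shows both widgets, enables input and disables character movement.
; Tab restores the mesh, removes the widgets, disables input, resets movement to walking and makes the note interactable again.
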(event `self.ReceiveBeginPlay`
  (set `self.InteractName` "pickup paper")
  (bind _returnvalue (`|CreateWidget` "/Game/Blueprints/Notes/WB_Note.WB_Note_C"))
  (set `self.NoteWidgetRef` _returnvalue)
  (bind _returnvalue_2 (`|CreateWidget` "/Game/Blueprints/Interact/WB_ViewText.WB_ViewText_C"))
  (bind _output_get (set `self.ViewWidgetRef` _returnvalue_2))
  (set `/Game/Blueprints/Interact/WB_ViewText.Name_3` "Press Tab to drop paper" _output_get)
  (`/Game/Blueprints/Notes/WB_Note.SetWidgetMaterial` (`self.NoteWidgetRef`) (`self.WidgetMaterial`)))

(event `/Game/Blueprints/Interact/Interface_Interact.Interact`
  (params (SMRef :type "StaticMeshComponent Object Reference"))
  (`SceneComponent.SetVisibility` (`self.MeshMaterial`) false false)
  (`UserWidget.AddToViewport` (`self.NoteWidgetRef`) 0)
  (`UserWidget.AddToViewport` (`self.ViewWidgetRef`) 0)
  (`self.EnableInput` (`GameplayStatics.GetPlayerController` 0))
  (set `self.CanInteract` false)
  (bind _asbp_first_person_character (cast `/Game/FirstPerson/Blueprints/BP_FirstPersonCharacter` (`GameplayStatics.GetPlayerCharacter` 0)))
  (`CharacterMovementComponent.DisableMovement` (`Character.CharacterMovement` _asbp_first_person_character)))

(event `Key|Tab`
  (params (Key :type "Key Structure"))
  (:`Pressed`
    (`SceneComponent.SetVisibility` (`self.MeshMaterial`) true false)
    (`Widget.RemoveFromParent` (`self.NoteWidgetRef`))
    (`Widget.RemoveFromParent` (`self.ViewWidgetRef`))
    (`self.DisableInput` (`GameplayStatics.GetPlayerController` 0) null)
    (set `self.CanInteract` true)
    (bind _asbp_first_person_character (cast `/Game/FirstPerson/Blueprints/BP_FirstPersonCharacter` (`GameplayStatics.GetPlayerCharacter` 0)))
    (`CharacterMovementComponent.SetMovementMode` (`Character.CharacterMovement` _asbp_first_person_character) "MOVE_Walking" 0)))

(fn `UserConstructionScript`)