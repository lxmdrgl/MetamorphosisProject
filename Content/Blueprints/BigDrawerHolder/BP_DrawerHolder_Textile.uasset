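; Interactable textile drawer cabinet whose drawers slide open and shut, and which topples when it becomes top-heavy.
; Interact toggles the chosen drawer along local X with a shared timeline, judging open or closed from its position, and counts open top and bottom drawers.
; Two open top drawers with no bottom drawer open trigger KnockOverDrawer, which lerps the cabinet between start and end transforms, also sliding Drawer1 out if closed.
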(event `KnockOverDrawer`
  (bind _relativelocation_x (`KismetMathLibrary.BreakVector` (`SceneComponent.RelativeLocation` (`self.Drawer_1`))))
  (`KismetSystemLibrary.PrintString` "Knock over drawer")
  (set `self.InteractOver` true)
  (if (`KismetMathLibrary.NearlyEqual_FloatFloat` _relativelocation_x (`self.DrawerStart`) 0.001)
    (set `self.SMRef` (`self.Drawer_1`))
    (`TimelineComponent.PlayFromStart` (`self.Timeline`))
    (bind (_direction _alpha) (`Timeline|T_KnockOverLocker` :!via `PlayFromStart` :!label _label)
      (:`Update`
        (`SceneComponent.K2_SetRelativeTransform` (`self.DrawerHolder`) (`KismetMathLibrary.TLerp` (`self.StartTransform`) (`self.EndTransform`) _alpha) false false)))
    (else
      (goto _label :!via `PlayFromStart`))))

(event `self.ReceiveBeginPlay`
  (bind _asbp_first_person_character (cast `/Game/FirstPerson/Blueprints/BP_FirstPersonCharacter` (`GameplayStatics.GetPlayerCharacter` 0)))
  (set `self.FPCharRef` _asbp_first_person_character)
  (set `self.InteractName` "interact with")
  (set `self.UsesMesh` true))

(event `/Game/Blueprints/Interact/Interface_Interact.Interact`
  (params (SMRef :type "StaticMeshComponent Object Reference"))
  (bind _smref (`self.SMRef`))
  (bind _smref_2 (`self.SMRef`))
  (bind _smref_3 (`self.SMRef`))
  (bind _smref_4 (`self.SMRef`))
  (bind _relativelocation_x (`KismetMathLibrary.BreakVector` (`SceneComponent.RelativeLocation` (`self.SMRef`))))
  (bind (_relativelocation_x_2 _relativelocation_y _relativelocation_z) (`KismetMathLibrary.BreakVector` (`SceneComponent.RelativeLocation` _smref_2)))
  (bind _returnvalue (and (== (`self.OpenTopCount`) 2) (== (`self.OpenBottomCount`) 0)))
  (bind _returnvalue_2 (or (== _smref (`self.Drawer_4`)) (== _smref (`self.Drawer_5`)) (== _smref (`self.Drawer_6`)) (== _smref (`self.Drawer_7`)) (== _smref (`self.Drawer_8`))))
  (set `self.SMRef` SMRef)
  (set `self.CanInteract` false)
  (`|ExecutionSequence`
    (:`then_0`
      (if (== (`StaticMeshComponent.StaticMesh` (`self.SMRef`)) "/Game/Blueprints/Desk/Drawer/SM_Desk_Drawer.SM_Desk_Drawer")
        (if (`KismetMathLibrary.NearlyEqual_FloatFloat` _relativelocation_x (`self.DrawerStart`))
          (`|ExecutionSequence`
            (:`then_0`
              (`TimelineComponent.SetPlayRate` (`self.Timeline`) 2.0)
              (bind (_direction _alpha) (`Timeline|Timeline` :!via `PlayFromStart` :!label _label_2)
                (:`Update`
                  (`SceneComponent.K2_SetRelativeLocation` _smref_2 (`KismetMathLibrary.MakeVector` (`KismetMathLibrary.Lerp` (`self.DrawerStart`) (`self.DrawerEnd`) _alpha) _relativelocation_y _relativelocation_z) false false))
                (:`Finished`
                  (set `self.CanInteract` true))))
            (:`then_1`
              (if _returnvalue_2
                (`/Engine/EditorBlueprintResources/StandardMacros.IncrementInt` (`self.OpenBottomCount`))))
            (:`then_2`
              (`|ExecutionSequence`
                (:`then_0`
                  (if (== (`self.SMRef`) (`self.Drawer_1`))
                    (`/Engine/EditorBlueprintResources/StandardMacros.IncrementInt` (`self.OpenTopCount`)
                      (:`  `
                        (if _returnvalue
                          (`self.KnockOverDrawer` :!label _label_3))))))
                (:`then_1`
                  (if (or (== _smref_3 (`self.Drawer_2`)) (== _smref_3 (`self.Drawer_3`)))
                    (`/Engine/EditorBlueprintResources/StandardMacros.IncrementInt` (`self.OpenTopCount`)
                      (:`  `
                        (if _returnvalue :!label _label_4
                          (set `self.InteractOver` false)
                          (`KismetSystemLibrary.Delay` 0.5)
                          (goto _label_3)))))))))
          (else
            (`|ExecutionSequence`
              (:`then_0`
                (goto _label_2 :!via `ReverseFromEnd`))
              (:`then_1`
                (if _returnvalue_2
                  (`/Engine/EditorBlueprintResources/StandardMacros.DecrementInt` (`self.OpenBottomCount`)
                    (:`  `
                      (goto _label_4)))))
              (:`then_2`
                (if (or (== _smref_4 (`self.Drawer_2`)) (== _smref_4 (`self.Drawer_3`)) (== _smref_4 (`self.Drawer_1`)))
                  (`/Engine/EditorBlueprintResources/StandardMacros.DecrementInt` (`self.OpenTopCount`)))))))
        (else
          (set `self.CanInteract` true))))))

(fn `UserConstructionScript`)