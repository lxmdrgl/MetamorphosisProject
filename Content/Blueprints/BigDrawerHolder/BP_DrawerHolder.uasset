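; BP_DrawerHolder is an interactable drawer holder whose desk drawers slide open and closed when interacted with.
; Interact receives the targeted static mesh component and only animates it if it uses the SM_Desk_Drawer mesh.
; Its relative X, compared to DrawerStart, decides whether a shared Timeline plays forward or reverses, lerping between start and end positions.
; CanInteract blocks further interaction until the Timeline finishes, or resets immediately for other meshes.
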(event `self.ReceiveBeginPlay`
  (bind _asbp_first_person_character (cast `/Game/FirstPerson/Blueprints/BP_FirstPersonCharacter` (`GameplayStatics.GetPlayerCharacter` 0)))
  (set `self.FPCharRef` _asbp_first_person_character)
  (set `self.InteractName` "interact with")
  (set `self.UsesMesh` true))

(event `/Game/Blueprints/Interact/Interface_Interact.Interact`
  (params (SMRef :type "StaticMeshComponent Object Reference"))
  (bind _smref (`self.SMRef`))
  (bind _relativelocation_x (`KismetMathLibrary.BreakVector` (`SceneComponent.RelativeLocation` (`self.SMRef`))))
  (bind (_relativelocation_x_2 _relativelocation_y _relativelocation_z) (`KismetMathLibrary.BreakVector` (`SceneComponent.RelativeLocation` _smref)))
  (set `self.SMRef` SMRef)
  (set `self.CanInteract` false)
  (if (== (`StaticMeshComponent.StaticMesh` (`self.SMRef`)) "/Game/Blueprints/Desk/Drawer/SM_Desk_Drawer.SM_Desk_Drawer")
    (if (`KismetMathLibrary.NearlyEqual_FloatFloat` _relativelocation_x (`self.DrawerStart`))
      (`TimelineComponent.SetPlayRate` (`self.Timeline`) 2.0)
      (bind (_direction _alpha) (`Timeline|Timeline` :!via `PlayFromStart` :!label _label)
        (:`Update`
          (`SceneComponent.K2_SetRelativeLocation` _smref (`KismetMathLibrary.MakeVector` (`KismetMathLibrary.Lerp` (`self.DrawerStart`) (`self.DrawerEnd`) _alpha) _relativelocation_y _relativelocation_z) false false))
        (:`Finished`
          (set `self.CanInteract` true)))
      (else
        (goto _label :!via `ReverseFromEnd`)))
    (else
      (set `self.CanInteract` true))))

(fn `UserConstructionScript`)