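; BP_Item is an interactable item Blueprint that supplies the prompt text for its interaction.
; GetName resolves that text by priority: NameSuperOveride first, then NameOveride, then a default "Press E to" prompt formatted with InteractName.
; When neither override is set and InteractOver is true, it returns empty text.
; The construction script is empty.
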(fn `Get Name`
  (returns (GetName :type Text))
  (if (`KismetTextLibrary.TextIsEmpty` (`self.NameSuperOveride`))
    (if (`KismetTextLibrary.TextIsEmpty` (`self.NameOveride`))
      (if (`self.InteractOver`)
        (set `self.ReturnName` "")
        (else
          (set `self.ReturnName` (`|FormatText` "Press E to {X}" (`self.InteractName`)))))
      (else
        (set `self.ReturnName` (`self.NameOveride`))))
    (else
      (set `self.ReturnName` (`self.NameSuperOveride`))))
  (return (`self.ReturnName`)))

(fn `UserConstructionScript`)