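; BP_Safe is an interactable safe that moves the player's view to a close-up of itself.
; Interact blends the camera to the safe, enables its input and the mouse cursor, locks look input and shows EndName through a WB_ViewText widget created at BeginPlay.
; Tab clears the text, blends back to the first-person character cached on collision overlap, and restores look input and interactability.
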(event `self.Collision.OnComponentBeginOverlap`
  (params (OverlappedComponent :type "PrimitiveComponent Object Reference") (OtherActor :type "Actor Object Reference") (OtherComp :type "PrimitiveComponent Object Reference") (OtherBodyIndex :type Integer) (bFromSweep :type Boolean) (SweepResult :type "HitResult Structure (by ref)"))
  (bind _asbp_first_person_character (cast `/Game/FirstPerson/Blueprints/BP_FirstPersonCharacter` OtherActor))
  (set `self.FPCharRef` _asbp_first_person_character))

(event `self.ReceiveBeginPlay`
  (bind _returnvalue (`GameplayStatics.GetPlayerController` 0))
  (set `self.ItemName` (`self.StartName`))
  (`self.DisableInput` _returnvalue)
  (bind _returnvalue_2 (`|CreateWidget` "/Game/Blueprints/Interact/WB_ViewText.WB_ViewText_C" _returnvalue))
  (bind _output_get (set `self.WidgetRef` _returnvalue_2))
  (`UserWidget.AddToViewport` _output_get 0))

(event `/Game/Blueprints/Interact/Interface_Interact.Interact`
  (bind _returnvalue (`GameplayStatics.GetPlayerController` 0))
  (set `self.CanInteract` false)
  (`PlayerController.SetViewTargetWithBlend` (`GameplayStatics.GetPlayerController` 0) self 0.5 "VTBlend_Linear" 0.0 false)
  (`KismetSystemLibrary.Delay` 0.5)
  (`self.EnableInput` _returnvalue)
  (set `PlayerController.bShowMouseCursor` true _returnvalue)
  (set `/Game/Blueprints/Interact/WB_ViewText.Name` (`self.EndName`) (`self.WidgetRef`))
  (`Controller.SetIgnoreLookInput` _returnvalue true))

(event `Key|Tab`
  (params (Key :type "Key Structure"))
  (bind _returnvalue (`GameplayStatics.GetPlayerController` 0))
  (bind _returnvalue_2 (`GameplayStatics.GetPlayerController` 0))
  (:`Pressed`
    (set `/Game/Blueprints/Interact/WB_ViewText.Name` "" (`self.WidgetRef`))
    (set `PlayerController.bShowMouseCursor` false _returnvalue_2)
    (`PlayerController.SetViewTargetWithBlend` _returnvalue_2 (`self.FPCharRef`) 0.5 "VTBlend_Linear" 0.0 false)
    (`KismetSystemLibrary.Delay` 0.5)
    (`self.DisableInput` _returnvalue)
    (set `self.CanInteract` true)
    (`Controller.SetIgnoreLookInput` _returnvalue false)))

(fn `UserConstructionScript`)