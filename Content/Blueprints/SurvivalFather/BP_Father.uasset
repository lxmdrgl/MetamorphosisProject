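; BP_Father is the father actor in SurvivalFather, which shifts between two fixed positions.
; FatherMove and MoveBack play and reverse the Movement timeline, whose Finished pin sets the lerped location, so it snaps rather than glides.
; SwitchMode, run at BeginPlay, starts a one-shot random-delay timer on Move, and DoorClosed cancels it.
; Move is empty and the probability-based FatherMove trigger is unwired, so the timer moves nothing.
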(event `FatherMove`
  (bind (_direction _alpha_value) (`Timeline|Movement` :!label _label)
    (:`Finished`
      (`self.K2_SetActorLocation` (`KismetMathLibrary.VLerp` (-270.0 -220.0 40.0) (-170.0 130.0 40.0) _alpha_value)))))

(event `Move Back`
  (goto _label :!via `Reverse`))

(event `DoorClosed`
  (`KismetSystemLibrary.K2_ClearAndInvalidateTimerHandle` (stale `Switch Mode` _returnvalue)))

(event `Switch Mode`
  (bind _returnvalue (`KismetSystemLibrary.K2_SetTimer` null "Move" (`KismetMathLibrary.RandomFloatInRange` 10.0 20.0))))

(event `self.ReceiveBeginPlay`
  (`self.Switch Mode`))

(fn `Move`)

(fn `UserConstructionScript`)