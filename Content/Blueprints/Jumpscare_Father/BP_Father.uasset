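; BP_Father is the jumpscare father actor, which can jump to a new position after a random delay unless the door closes first.
; BeginPlay calls SwitchMode to start a one-shot Move timer, and DoorClosed clears it.
; Move teleports only if a random float exactly equals its upper bound ProbMove, so it rarely fires for nonzero values.
; The Lerp alpha is fixed at one, giving a constant destination, logged as "moved".
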(event `DoorClosed`
  (`KismetSystemLibrary.K2_ClearAndInvalidateTimerHandle` (stale `Switch Mode` _returnvalue)))

(event `Switch Mode`
  (bind _returnvalue (`KismetSystemLibrary.K2_SetTimer` null "Move" (`KismetMathLibrary.RandomFloatInRange` 10.0 20.0))))

(event `self.ReceiveBeginPlay`
  (`self.Switch Mode`))

(fn `Move`
  (bind _probmove (`self.ProbMove`))
  (if (== _probmove (`KismetMathLibrary.RandomFloatInRange` 0.0 _probmove))
    (`self.K2_SetActorLocation` (`KismetMathLibrary.VLerp` (-270.0 -220.0 40.0) (-170.0 130.0 40.0) 1.0))
    (`KismetSystemLibrary.PrintString` "moved")))

(fn `UserConstructionScript`)