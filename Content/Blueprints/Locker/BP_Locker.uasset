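; BP_Locker is an interactable hiding locker that the first-person player enters and leaves, notifying BP_BasicAI_2 both ways.
; Interact freezes, hides and disables collision on the player, blends the view to the locker, swings the door, then shows a WB_ViewText prompt.
; Tab removes the prompt, replays the door swing, blends the view back and, after a delay, restores the player.
; A position-tween path for the character is left unconnected.
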(event `TweenCharacter`
  (`CharacterMovementComponent.DisableMovement` (`Character.CharacterMovement` (`self.FPCharRef`)))
  (`Controller.SetIgnoreLookInput` (`GameplayStatics.GetPlayerController` 0) true)
  (`self.SetActorHiddenInGame` (`self.FPCharRef`) true)
  (`self.SetActorEnableCollision` (`self.FPCharRef`) false)
  (`self.HideInLocker`))

(event `self.ReceiveBeginPlay`
  (set `self.UsesMesh` true)
  (set `self.InteractName` (`self.StartName`))
  (bind _asbp_first_person_character (cast `/Game/FirstPerson/Blueprints/BP_FirstPersonCharacter` (`GameplayStatics.GetPlayerCharacter` 0)))
  (set `self.FPCharRef` _asbp_first_person_character)
  (`TimelineComponent.SetPlayRate` (`self.Timeline`) 1.5)
  (`TimelineComponent.SetPlayRate` (`self.T_OpenDoor`) 1.5))

(event `/Game/Blueprints/Interact/Interface_Interact.Interact`
  (params (SMRef :type "StaticMeshComponent Object Reference"))
  (if (`self.CanInteract`)
    (bind _returnvalue (`GameplayStatics.GetActorOfClass` "/Game/AI/BasicAI_2/BP_BasicAI_2.BP_BasicAI_2_C"))
    (`/Game/AI/BasicAI_2/BP_BasicAI_2.StartHideInLocker` _returnvalue)
    (set `self.CanInteract` false)
    (`self.TweenCharacter`)))

(event `HideInLocker`
  (bind _returnvalue (`GameplayStatics.GetPlayerController` 0))
  (`PlayerController.SetViewTargetWithBlend` (`GameplayStatics.GetPlayerController` 0) self 0.5 "VTBlend_Linear" 0.0 false)
  (bind (_direction _alpha) (`Timeline|T_OpenDoor` :!via `PlayFromStart`)
    (:`Update`
      (`SceneComponent.K2_SetRelativeRotation` (`self.LockerDoor`) (`KismetMathLibrary.MakeRotator` 0.0 0.0 (`KismetMathLibrary.Lerp` 0.0 -150.0 _alpha)) false false))
    (:`Finished`
      (`self.EnableInput` _returnvalue)
      (bind _returnvalue_2 (`|CreateWidget` "/Game/Blueprints/Interact/WB_ViewText.WB_ViewText_C" _returnvalue))
      (bind _output_get (set `self.WidgetRef` _returnvalue_2))
      (set `/Game/Blueprints/Interact/WB_ViewText.Name` (`self.EndName`) _output_get)
      (`UserWidget.AddToViewport` (`self.WidgetRef`) 0))))

(event `Key|Tab`
  (params (Key :type "Key Structure"))
  (:`Pressed`
    (`self.DisableInput` null)
    (`Widget.RemoveFromParent` (`self.WidgetRef`))
    (`|ExecutionSequence`
      (:`then_0`
        (bind (_direction _alpha) (`Timeline|Timeline` :!via `PlayFromStart`)
          (:`Update`
            (`SceneComponent.K2_SetRelativeRotation` (`self.LockerDoor`) (`KismetMathLibrary.MakeRotator` 0.0 0.0 (`KismetMathLibrary.Lerp` 0.0 -150.0 _alpha)) false false))))
      (:`then_1`
        (`KismetSystemLibrary.Delay` 0.25)
        (`PlayerController.SetViewTargetWithBlend` (`GameplayStatics.GetPlayerController` 0) (`self.FPCharRef`) 0.5 "VTBlend_Linear" 0.0 false))
      (:`then_2`
        (`KismetSystemLibrary.Delay` 1.0)
        (set `self.CanInteract` true)
        (`Controller.SetIgnoreLookInput` (`GameplayStatics.GetPlayerController` 0) false)
        (`CharacterMovementComponent.SetMovementMode` (`Character.CharacterMovement` (`self.FPCharRef`)) "MOVE_Walking" 0)
        (`self.SetActorHiddenInGame` (`self.FPCharRef`) false)
        (`self.SetActorEnableCollision` (`self.FPCharRef`) true)
        (bind _returnvalue (`GameplayStatics.GetActorOfClass` "/Game/AI/BasicAI_2/BP_BasicAI_2.BP_BasicAI_2_C"))
        (`/Game/AI/BasicAI_2/BP_BasicAI_2.EndHideInLocker` _returnvalue)))))

(fn `Get Name`
  (returns (GetName :type Text))
  (return ""))

(fn `UserConstructionScript`)