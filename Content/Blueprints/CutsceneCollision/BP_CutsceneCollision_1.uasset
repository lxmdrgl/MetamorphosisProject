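; BP_CutsceneCollision_1 is a trigger volume that locks player movement and runs a screen fade on overlap, apparently as a cutscene lead-in.
; BeginPlay caches the first-person character and creates the fade widget.
; Any overlap on Collision disables that character's movement, then plays the widget's FadeOut animation reversed and forward, separated by delays, before removing it.
; It never restores movement or starts a cutscene itself.
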(event `self.ReceiveBeginPlay`
  (bind _asbp_first_person_character (cast `/Game/FirstPerson/Blueprints/BP_FirstPersonCharacter` (`GameplayStatics.GetPlayerCharacter` 0)))
  (set `self.FPCharRef` _asbp_first_person_character)
  (bind _returnvalue (`|CreateWidget` "/Game/Blueprints/Interact/WB_Fade.WB_Fade_C"))
  (set `self.FadeWidgetRef` _returnvalue))

(event `self.Collision.OnComponentBeginOverlap`
  (params (OverlappedComponent :type "PrimitiveComponent Object Reference") (OtherActor :type "Actor Object Reference") (OtherComp :type "PrimitiveComponent Object Reference") (OtherBodyIndex :type Integer) (bFromSweep :type Boolean) (SweepResult :type "HitResult Structure (by ref)"))
  (bind _fadewidgetref (`self.FadeWidgetRef`))
  (bind _fadewidgetref_2 (`self.FadeWidgetRef`))
  (`CharacterMovementComponent.DisableMovement` (`Character.CharacterMovement` (`self.FPCharRef`)))
  (`UserWidget.AddToViewport` (`self.FadeWidgetRef`) 0)
  (`UserWidget.PlayAnimationReverse` _fadewidgetref (`/Game/Blueprints/Interact/WB_Fade.FadeOut` _fadewidgetref) 1.0 true)
  (`KismetSystemLibrary.Delay` 1.0)
  (`UserWidget.PlayAnimationForward` _fadewidgetref_2 (`/Game/Blueprints/Interact/WB_Fade.FadeOut` _fadewidgetref_2) 1.0 false)
  (`KismetSystemLibrary.Delay` 0.95)
  (`Widget.RemoveFromParent` (`self.FadeWidgetRef`)))

(fn `UserConstructionScript`)