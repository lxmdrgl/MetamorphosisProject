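; Enemy AI character that hunts the player, reacts to locker hiding and restarts the level on capture.
; Locker events write blackboard flags, sending the AI to the locker if the player is its current target.
; AttackPlayer sphere-traces ahead and, on hitting the player, aborts the behavior tree, freezes them, plays capture effects and a fade, then reloads the level.
; Teleport, blackboard-clearing and player-start respawn chains are unconnected.
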(event `StartHideInLocker`
  (bind _blackboard (`AIController.Blackboard` (`AIBlueprintHelperLibrary.GetAIController` self)))
  (`|ExecutionSequence`
    (:`then_0`
      (if (== (`BlackboardComponent.GetValueAsObject` _blackboard "TargetActor") (`GameplayStatics.GetPlayerCharacter` 0))
        (`BlackboardComponent.SetValueAsBool` _blackboard "GoToLocker" true)))
    (:`then_1`
      (`BlackboardComponent.SetValueAsBool` _blackboard "isPlayerInLocker?" true))))

(event `EndHideInLocker`
  (`BlackboardComponent.SetValueAsBool` (`AIController.Blackboard` (`AIBlueprintHelperLibrary.GetAIController` self)) "IsPlayerInLocker?" false))

(event `AttackPlayer`
  (bind _returnvalue (`self.K2_GetActorLocation`))
  (bind _widgetref (`self.WidgetRef`))
  (bind (_outhit _returnvalue_2) (`KismetSystemLibrary.SphereTraceSingleForObjects` :`Start` _returnvalue :`End` (+ _returnvalue (* (`KismetMathLibrary.GetForwardVector` (`self.K2_GetActorRotation`)) 50.0)) :`Radius` 120.0 :`ObjectTypes` (`|MakeArray` "ObjectTypeQuery3" :!type "EObjectTypeQuery Enum") :`DrawDebugType` "ForDuration"))
  (if _returnvalue_2
    (bind _asbp_first_person_character (cast `/Game/FirstPerson/Blueprints/BP_FirstPersonCharacter` (`.HitActor` (`GameplayStatics.BreakHitResult` _outhit))))
    (`BlackboardComponent.SetValueAsBool` (`AIController.Blackboard` (`AIBlueprintHelperLibrary.GetAIController` self)) "AbortBT" true)
    (`/Engine/EditorBlueprintResources/StandardMacros.DoOnce` false :!label _label
      (:`Completed`
        (`CharacterMovementComponent.DisableMovement` (`Character.CharacterMovement` _asbp_first_person_character))
        (`GameplayStatics.PlaySound2D` "/Game/Blueprints/Dialogue/Replica/Sounds/Captured_Cue.Captured_Cue" 1.0 1.0 0.0 null null)
        (`self.PlayAnimMontage` "/Game/AI/BasicAI_2/Animations/Zombie_Attack_Chief_Montage.Zombie_Attack_Chief_Montage" 1.5)
        (`KismetSystemLibrary.Delay` 1.0)
        (`UserWidget.AddToViewport` _widgetref 0)
        (`UserWidget.PlayAnimationReverse` _widgetref (`/Game/Blueprints/Interact/WB_Fade.FadeOut` _widgetref) 1.0 false)
        (`KismetSystemLibrary.Delay` 1.0)
        (bind _returnvalue_3 (`GameplayStatics.GetCurrentLevelName` true))
        (`GameplayStatics.OpenLevel` (`KismetStringLibrary.Conv_StringToName` _returnvalue_3) false)
        (bind _asnew_game_instance (cast `/Game/Blueprints/NewGameInstance` (`GameplayStatics.GetGameInstance`))
          (:`then`
            (set `/Game/Blueprints/NewGameInstance.PlayOpening_1` false _asnew_game_instance)
            (goto _label :!via `Reset`))
          (:`CastFailed`
            (goto _label :!via `Reset`)))))))

(event `self.ReceiveBeginPlay`
  (bind _returnvalue (`|CreateWidget` "/Game/Blueprints/Interact/WB_Fade.WB_Fade_C"))
  (set `self.WidgetRef` _returnvalue))

(fn `UserConstructionScript`)