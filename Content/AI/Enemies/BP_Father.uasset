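; BP_Father is an AI enemy that feeds player position and door state to its AI controller's Blackboard.
; Every Tick it fetches the Blackboard and writes PlayerLocation from player controller 0's actor location, rather than the pawn's.
; DoorClosed and DoorOpen events set separate IsDoorClosed and IsDoorOpen keys to true, and neither key is cleared here.
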(event `self.ReceiveTick`
  (params (DeltaSeconds :type "Float (single-precision)"))
  (bind _output_get (set `self.Blackboard` (`AIController.Blackboard` (`AIBlueprintHelperLibrary.GetAIController` self))))
  (`BlackboardComponent.SetValueAsVector` _output_get "PlayerLocation" (`self.K2_GetActorLocation` (`GameplayStatics.GetPlayerController` 0))))

(event `DoorClosed`
  (`BlackboardComponent.SetValueAsBool` (`self.Blackboard`) "IsDoorClosed" true))

(event `DoorOpen`
  (`BlackboardComponent.SetValueAsBool` (`self.Blackboard`) "IsDoorOpen" true))

(fn `UserConstructionScript`)